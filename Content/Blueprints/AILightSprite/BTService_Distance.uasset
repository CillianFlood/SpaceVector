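; Behavior tree service for the AI light sprite that tracks its distance to the player.
; On each tick it reads the player actor from the blackboard and writes the length between the controlled pawn and that actor into a float key.
; When the player reference is invalid, it writes zero instead.
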(event EventTick
  (params (OwnerActor :type Actor%20Object%20Reference) (DeltaSeconds :type Float%20%28single-precision%29))
  (bind _playerobject (Variables|Default|GetPlayerObject))
  (bind _playerspriedistance (Variables|Default|GetPlayerSprieDistance))
  (bind _returnvalue (AI|BehaviorTree|GetBlackboardValueasActor _playerobject))
  (bind _asaicontroller (Utilities|Casting|CastToAIController OwnerActor))
  (Utilities|IsValid _returnvalue
    (:Is%20Valid
      (Class|BTFunctionLibrary|SetBlackboardValueasFloat _playerspriedistance (Math|Vector|VectorLength (- (Transformation|GetActorLocation (Pawn|GetControlledPawn _asaicontroller)) (Transformation|GetActorLocation _returnvalue)))))
    (:Is%20Not%20Valid
      (Class|BTFunctionLibrary|SetBlackboardValueasFloat _playerspriedistance 0.0))))