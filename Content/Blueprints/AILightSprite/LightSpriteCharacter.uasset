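; LightSpriteCharacter is a turret enemy that tracks the player's yaw, fires projectiles and deals contact damage at close range.
; Looping timers drive firing, the proximity check and a FlipFlop barrier that swaps the turret material.
; Projectile hits cost health only while the barrier is down; surviving one toggles the barrier and restarts its timer.
; Death spawns a life pickup and explosion; Tick's search rotation branch is unreachable.
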(event Custom|TurretFire
  ;[1 1 1] Firing
  (Game|SpawnActorfromClass "/Game/Blueprints/AILightSprite/TurretProjectile.TurretProjectile_C" (Transformation|GetSocketTransform (Variables|Default|GetTurret) "Socket" "RTS_World") false 0))

(event Custom|ContactTimer
  ;[1 1 1] DamagePlayerOnContact
  (if (<= (Math|Vector|VectorLength (- (Transformation|GetActorLocation) (Transformation|GetActorLocation (Game|GetPlayerCharacter 0)))) 2.5e+02)
    (Game|Damage|ApplyDamage (Game|GetPlayerCharacter 0) 1.0 0 self "/Script/Engine.DamageType")))

(event Custom|Barrier
  (bind _turret (Variables|Default|GetTurret))
  ;[1 1 1] Barrier
  (Utilities|FlowControl|FlipFlop
    (:A
      (Rendering|Material|SetMaterial _turret 0 "/Engine/EngineDebugMaterials/BoneWeightMaterial.BoneWeightMaterial")
      (Variables|Default|SetBarrierDown false))
    (:B
      (Rendering|Material|SetMaterial _turret 0 "/Engine/Engine_MI_Shaders/MI_Shader_BaseTileEx.MI_Shader_BaseTileEx")
      (Variables|Default|SetBarrierDown true))))

(event EventHit
  (params (MyComp :type Primitive%20Component%20Object%20Reference) (Other :type Actor%20Object%20Reference) (OtherComp :type Primitive%20Component%20Object%20Reference) (bSelfMoved :type Boolean) (HitLocation :type Vector :default "0, 0, 0") (HitNormal :type Vector :default "0, 0, 0") (NormalImpulse :type Vector :default "0, 0, 0") (Hit :type Hit%20Result%20Structure%20%28by%20ref%29))
  (bind _returnvalue (Transformation|GetActorLocation))
  (bind _turret (Variables|Default|GetTurret))
  (bind (_x _y _z) (Math|Vector|BreakVector _returnvalue))
  (bind _returnvalue_2 (+ 1.5e+02 _z))
  (bind _returnvalue_3 (Math|Vector|MakeVector _x _y _returnvalue_2))
  (bind _returnvalue_4 (Math|Conversions|ToTransform(Vector) _returnvalue_3))
  ;[1 1 1] Damage Calc
  (bind _outactors (Actor|GetAllActorsOfClass "/Game/Blueprints/Projectile.Projectile_C"))
  (for _array_element _outactors
    (bind _asprojectile_c (Utilities|Casting|CastToProjectile _array_element))
    (if (== Other _asprojectile_c)
      (if (Variables|Default|GetBarrierDown)
        (Variables|Default|SetHealth (- (Variables|Default|GetHealth) 1))
        (Actor|DestroyActor Other)
        (if (<= (Variables|Default|GetHealth) 0)
          (Game|SpawnActorfromClass "/Game/Blueprints/PickUps/LifePickup.LifePickup_C" _returnvalue_4 false 0)
          (Game|SpawnActorfromClass "/Game/Blueprints/SilentExplosion.SilentExplosion_C" _returnvalue_4 false 0)
          (Actor|DestroyActor)
          (else
            ;[1 1 1] Barrier
            (Utilities|Time|SetTimerbyFunctionName 0 "Barrier" 5.0 true)
            (Utilities|FlowControl|FlipFlop
              (:A
                (Rendering|Material|SetMaterial _turret 0 "/Engine/EngineDebugMaterials/BoneWeightMaterial.BoneWeightMaterial")
                (Variables|Default|SetBarrierDown false))
              (:B
                (Rendering|Material|SetMaterial _turret 0 "/Engine/Engine_MI_Shaders/MI_Shader_BaseTileEx.MI_Shader_BaseTileEx")
                (Variables|Default|SetBarrierDown true)))))))))

(event EventBeginPlay
  ;[1 1 1] SetUp
  (Utilities|Time|SetTimerbyFunctionName 0 "Barrier" 5.0 true)
  (Utilities|Time|SetTimerbyFunctionName 0 "TurretFire" 2.0 true)
  (Utilities|Time|SetTimerbyFunctionName 0 "ContactTimer" 1.0 true))

(event EventTick
  (params (DeltaSeconds :type Float%20%28single-precision%29))
  (bind _turret (Variables|Default|GetTurret))
  (if true
    ;[1 1 1] FollowPlayer
    (Transformation|SetWorldRotation _turret (Math|Interpolation|RInterpTo (Transformation|GetWorldRotation _turret) (Class|KismetMathLibrary|MakeRot 0.0 (+ (.Yaw (Class|KismetMathLibrary|BreakRot (Math|Rotator|FindLookatRotation (Transformation|GetWorldLocation _turret) (Transformation|GetActorLocation (Game|Player|GetPlayerPawn 0))))) 1.8e+02) 0.0) DeltaSeconds 5.0) false)
    (else
      ;[1 1 1] Search
      (Transformation|AddActorLocalRotation "0,1.000000, 0" false))))

(fn ConstructionScript)