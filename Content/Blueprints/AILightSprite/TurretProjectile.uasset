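; Turret projectile actor that damages the player on a nearby impact.
; A timer started at BeginPlay destroys it after a fixed lifespan.
; On Hit, it checks distance to the player character rather than the struck actor, applying damage and destroying itself only if the player is within range.
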(event Custom|LifeSpan
  ;[1 1 1] Collision
  (Actor|DestroyActor))

(event EventHit
  (params (MyComp :type Primitive%20Component%20Object%20Reference) (Other :type Actor%20Object%20Reference) (OtherComp :type Primitive%20Component%20Object%20Reference) (bSelfMoved :type Boolean) (HitLocation :type Vector :default "0, 0, 0") (HitNormal :type Vector :default "0, 0, 0") (NormalImpulse :type Vector :default "0, 0, 0") (Hit :type Hit%20Result%20Structure%20%28by%20ref%29))
  ;[1 1 1] Collision
  (if (<= (Math|Vector|VectorLength (- (Transformation|GetActorLocation) (Transformation|GetActorLocation (Game|GetPlayerCharacter 0)))) 1.5e+02)
    (Game|Damage|ApplyDamage (Game|GetPlayerCharacter 0) 1.0 0 self "/Script/Engine.DamageType")
    (Actor|DestroyActor)))

(event EventBeginPlay
  ;[1 1 1] Collision
  (Utilities|Time|SetTimerbyFunctionName 0 "LifeSpan" 15.0))

(fn ConstructionScript)