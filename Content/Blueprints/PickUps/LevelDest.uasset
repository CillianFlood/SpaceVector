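; LevelDest is a pickup-folder actor, apparently a level destination marker, that animates as a spinning visual with no overlap or level-change logic.
; Each Tick yaws the Torus and Other components one degree in opposite directions, so the speed depends on frame rate.
; Tick also plays a timeline whose update applies a zero local offset, leaving the actor in place.
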(event EventTick
  (params (DeltaSeconds :type Float%20%28single-precision%29))
  (bind _torus (Variables|Default|GetTorus))
  (bind _other (Variables|Default|GetOther))
  (bind _returnvalue (Transformation|GetWorldRotation _other))
  (bind _returnvalue_2 (Transformation|GetWorldRotation _torus))
  (bind (_pitch _yaw _roll) (Class|KismetMathLibrary|BreakRot _returnvalue))
  (bind (_pitch_2 _yaw_2 _roll_2) (Class|KismetMathLibrary|BreakRot _returnvalue_2))
  (Transformation|SetWorldRotation _torus (Class|KismetMathLibrary|MakeRot _pitch_2 (+ _yaw_2 1.0) _roll_2) false)
  (Transformation|SetWorldRotation _other (Class|KismetMathLibrary|MakeRot _pitch (- _yaw 1.0) _roll) false)
  (Timeline|Timeline_0 Play
    (:Update
      (Transformation|AddActorLocalOffset "0, 0, 0" false))))

(fn ConstructionScript)