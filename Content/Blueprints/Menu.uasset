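; Menu Blueprint that serves as a level select, using clickable static mesh components as buttons.
; Each of six meshes opens its own level by name on click: Tutorial, three numbered levels, Survival or Boss.
; The gamepad Special Right and bottom face buttons share the Level1 load with its mesh click.
; A Quit Game node is present but not connected to any event.
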(event OnClicked(StaticMesh1)
  (params (TouchedComponent :type Primitive%20Component%20Object%20Reference))
  (Game|OpenLevel(byName) "Tutorial"))

(event OnClicked(StaticMesh2)
  (params (TouchedComponent :type Primitive%20Component%20Object%20Reference))
  (Game|OpenLevel(byName) "Survival"))

(event OnClicked(StaticMesh4)
  (params (TouchedComponent :type Primitive%20Component%20Object%20Reference))
  (Game|OpenLevel(byName) "Level2"))

(event OnClicked(StaticMesh3)
  (params (TouchedComponent :type Primitive%20Component%20Object%20Reference))
  (Game|OpenLevel(byName) "Level3"))

(event OnClicked(StaticMesh6)
  (params (TouchedComponent :type Primitive%20Component%20Object%20Reference))
  (Game|OpenLevel(byName) "Boss"))

(event OnClicked(StaticMesh5)
  (params (TouchedComponent :type Primitive%20Component%20Object%20Reference))
  (Game|OpenLevel(byName) "Level1"))

(event Input|KeyboardEvents|Escape)

(event Input|GamepadEvents|GamepadSpecialRight
  (:Pressed
    (Game|OpenLevel(byName) "Level1")))

(event Input|GamepadEvents|GamepadFaceButtonBottom
  (:Pressed
    (Game|OpenLevel(byName) "Level1")))

(fn ConstructionScript)