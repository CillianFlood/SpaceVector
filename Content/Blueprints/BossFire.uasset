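; BossFire is a boss projectile that flies toward the player's position captured at spawn, without homing afterward.
; BeginPlay sets its rotation, stores that position and starts a lifespan timer that destroys it.
; Tick eases it toward the stored point with a delta-scaled lerp, using a distance check instead of collision to damage the player and destroy itself.
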(event Custom|LifeSpan
  ;[1 1 1] Destroy
  (Actor|DestroyActor))

(event EventBeginPlay
  ;[1 1 1] SetUp
  (Transformation|SetActorRotation (Math|Rotator|FindLookatRotation (Math|Vector|Lerp(Vector) (Transformation|GetActorLocation) (Variables|Default|GetPlayerLoc) (* (stale EventTick DeltaSeconds) (Variables|Default|GetSpeed))) (Variables|Default|GetPlayerLoc)))
  (Variables|Default|SetPlayerLoc (Transformation|GetActorLocation (Game|GetPlayerCharacter 0)))
  (Utilities|Time|SetTimerbyFunctionName 0 "LifeSpan" 15.0))

(event EventTick
  (params (DeltaSeconds :type Float%20%28single-precision%29))
  (bind _returnvalue (Transformation|GetActorLocation))
  ;[1 1 1] Movement
  (if (== (Game|GetPlayerCharacter 0) 0)
    (Actor|DestroyActor)
    (else
      (Transformation|SetActorLocation (Math|Vector|Lerp(Vector) _returnvalue (Variables|Default|GetPlayerLoc) (* DeltaSeconds (Variables|Default|GetSpeed))) false)
      ;[1 1 1] Apply Damage
      (if (<= (Math|Vector|VectorLength (- _returnvalue (Transformation|GetActorLocation (Game|GetPlayerCharacter 0)))) 1.5e+02)
        (Game|Damage|ApplyDamage (Game|GetPlayerCharacter 0) 1.0 0 self "/Script/Engine.DamageType")
        (Actor|DestroyActor)))))

(fn ConstructionScript)