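; LightSprite is a short-lived, constantly spinning actor that drifts after the player character and destroys itself after 30 seconds.
; Each Tick, when it is at a distance, a Timeline adds a local offset while a lerp pulls it toward the player at a randomized speed.
; Up close, it instead applies local offsets from the player-to-sprite direction plus that speed, so the spinning local frame continually turns its path.
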(event Custom|LifeSpan
  ;[1 1 1] SetUp
  (Actor|DestroyActor))

(event EventTick
  (params (DeltaSeconds :type Float%20%28single-precision%29))
  (bind _returnvalue (Transformation|GetActorLocation))
  (bind _returnvalue_2 (Game|GetPlayerCharacter 0))
  (bind _returnvalue_3 (Transformation|GetActorLocation _returnvalue_2))
  (bind _returnvalue_4 (Class|KismetMathLibrary|GetDirectionVector _returnvalue_3 _returnvalue))
  (bind _returnvalue_5 (Math|Vector|RotateVectorAroundAxis _returnvalue_4 0.0 "90.000000,0.000000,0.000000"))
  (bind (_x _y _z) (Math|Vector|BreakVector _returnvalue_5))
  ;[1 1 1] Movement
  (Transformation|AddActorLocalRotation "1.000000,1.000000,1.000000" false)
  (if (>= (Math|Vector|VectorLength (- _returnvalue _returnvalue_3)) 1.5e+02)
    (bind _newtrack_0 (Timeline|Timeline_0 Play)
      (:Update
        (Transformation|AddActorLocalOffset _newtrack_0 false)
        (Transformation|SetActorLocation (Math|Vector|Lerp(Vector) _returnvalue _returnvalue_3 (* DeltaSeconds (Variables|Default|GetSpeed))) false)))
    (else
      (Class|Actor|AddActorLocalTransform (Math|Conversions|ToTransform(Vector) (Math|Vector|MakeVector (+ _x (Variables|Default|GetSpeed)) _y _z)) false))))

(event EventBeginPlay
  ;[1 1 1] SetUp
  (Utilities|Time|SetTimerbyFunctionName 0 "LifeSpan" 3e+01)
  (Variables|Default|SetSpeed (Math|Random|RandomFloatinRange 0.1 0.9)))

(fn ConstructionScript)