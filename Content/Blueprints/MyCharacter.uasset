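; Player character Blueprint with a fuel-limited jetpack, health, score, checkpoints, music and pause controls.
; Tick handles game over, death, fall respawn at the last checkpoint and jetpack launches, while a looping timer refuels when grounded or air refuel is unlocked.
; Overlaps identify pickups through nested class searches to heal, upgrade fuel or jump power, spawn a pointer, or set checkpoints.
; Looping timers replay music and heartbeat, with a separate boss-map track.
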(event Custom|Refueler
  ;[1 1 1] Refueling
  (if (and (or (Math|Boolean|Equal(Boolean) (Variables|Default|GetAirRefuel) true) (== (.Z (Math|Vector|BreakVector (Transformation|GetVelocity (Game|GetPlayerCharacter 0)))) 0.0)) (Math|Boolean|Equal(Boolean) (Variables|Default|GetJetPack) false))
    (if (<= (Variables|Default|GetFuel) (Variables|Default|GetMaxFuel))
      (Variables|Default|SetFuel (+ (Variables|Default|GetFuel) 1)))))

(event Custom|HeartBeatTimer
  ;[1 1 1] Music
  (bind _returnvalue (Class|GameplayStatics|PlaySoundAttached "/Game/Audio/Heartbeat.Heartbeat" (Variables|Character|GetMesh))))

(event Custom|BossTimer
  ;[1 1 1] Music
  (bind _returnvalue (Class|GameplayStatics|PlaySoundAttached "/Game/Audio/Boss.Boss" (Variables|Character|GetMesh) "None" "0, 0, 0" "EAttachLocation::KeepRelativeOffset" false 0.3))
  (Utilities|Time|SetTimerbyFunctionName 0 "BossTimer" 1.5e+02 true))

(event Custom|MusicTimer
  (bind _mesh (Variables|Character|GetMesh))
  ;[1 1 1] Music
  (bind _returnvalue (Class|GameplayStatics|PlaySoundAttached "/Game/Audio/02.02" _mesh "None" "0, 0, 0" "EAttachLocation::KeepRelativeOffset" false 0.3))
  (bind _returnvalue_2 (Class|GameplayStatics|PlaySoundAttached "/Game/Audio/Heartbeat.Heartbeat" _mesh)))

(event EventBeginPlay
  (bind _mesh (Variables|Character|GetMesh))
  ;[1 1 1] Set Up
  (Variables|Default|SetCheckPoint (Transformation|GetActorLocation))
  (Variables|Default|SetStartRot (Transformation|GetActorRotation))
  (Utilities|Time|SetTimerbyFunctionName 0 "MusicTimer" 1.9e+02 true)
  (Utilities|Time|SetTimerbyFunctionName 0 "HeartBeatTimer" 6e+01 true)
  (Utilities|Time|SetTimerbyFunctionName 0 "Refueler" 0.05 true)
  ;[1 1 1] Music
  (bind _returnvalue (Class|MyProjectGameMode|GetCurrentMapReference (Game|GetGameMode)))
  (if (Utilities|Enum|Equal(Enum) _returnvalue "Boss")
    (bind _returnvalue_2 (Class|GameplayStatics|PlaySoundAttached "/Game/Audio/Boss.Boss" _mesh "None" "0, 0, 0" "EAttachLocation::KeepRelativeOffset" false 0.3))
    (Utilities|Time|SetTimerbyFunctionName 0 "BossTimer" 1.5e+02 true)
    (else
      (bind _returnvalue_3 (Class|GameplayStatics|PlaySoundAttached "/Game/Audio/02.02" _mesh "None" "0, 0, 0" "EAttachLocation::KeepRelativeOffset" false 0.3))
      (bind _returnvalue_4 (Class|GameplayStatics|PlaySoundAttached "/Game/Audio/Heartbeat.Heartbeat" _mesh)))))

(event EventAnyDamage
  (params (Damage :type Float%20%28single-precision%29) (DamageType :type Damage%20Type%20Object%20Reference) (InstigatedBy :type Controller%20Object%20Reference) (DamageCauser :type Actor%20Object%20Reference))
  ;[1 1 1] Damage Calculation
  (Variables|Default|SetHealth (- (Variables|Default|GetHealth) (Math|Float|Floor Damage)))
  (Class|PlayerController|ClientPlayCameraShake (Game|GetPlayerController 0) "/Game/Blueprints/PlayerDamage.PlayerDamage_C" 5.0 "ECameraAnimPlaySpace::CameraLocal" "0, 0, 0")
  (Audio|Components|Audio|Stop (stale _returnvalue))
  (bind _returnvalue (Class|GameplayStatics|PlaySoundAttached "/Game/Audio/Heavy_Breathing.Heavy_Breathing" (Variables|Character|GetMesh))))

(event EventActorBeginOverlap
  (params (OtherActor :type Actor%20Object%20Reference))
  (bind _mesh (Variables|Character|GetMesh))
  ;[1 1 1] PickUpCollision
  (bind _outactors (Actor|GetAllActorsOfClass "/Game/Blueprints/PickUps/LifePickup.LifePickup_C"))
  (for _array_element _outactors
    (bind _aslifepickup_c (Utilities|Casting|CastToLifePickup _array_element))
    (if (== OtherActor _aslifepickup_c)
      (if (>= 4 (Math|Float|Floor (Math|Conversions|ToFloat(Integer) (Variables|Default|GetHealth))))
        (Variables|Default|SetHealth (+ (Variables|Default|GetHealth) 1))
        (Development|PrintString "Health Restored")
        (Class|GameplayStatics|PlaySoundAttached "/Game/Audio/HealthRestore.HealthRestore" _mesh)
        (Actor|DestroyActor OtherActor :!label _label)
        (else
          (Development|PrintString "Health is at maximum")))
      (else
        (bind _outactors_2 (Actor|GetAllActorsOfClass "/Game/Blueprints/PickUps/AirRefuel.AirRefuel_C"))
        (for _array_element_2 _outactors_2
          (bind _asairrefuel_c (Utilities|Casting|CastToAirRefuel _array_element_2))
          (if (== OtherActor _asairrefuel_c)
            (Variables|Default|SetAirRefuel true)
            (Development|PrintString "Air Refuel Enabled")
            (Class|GameplayStatics|PlaySoundAttached "/Game/Audio/AirRefueler.AirRefueler" _mesh)
            (goto _label)
            (else
              (bind _outactors_3 (Actor|GetAllActorsOfClass "/Game/Blueprints/PickUps/FuelExpansion.FuelExpansion_C"))
              (for _array_element_3 _outactors_3
                (bind _asfuelexpansion_c (Utilities|Casting|CastToFuelExpansion _array_element_3))
                (if (== OtherActor _asfuelexpansion_c)
                  (Variables|Default|SetMaxFuel 199)
                  (Variables|Default|SetFuel (Variables|Default|GetMaxFuel))
                  (Development|PrintString "Jet Pack Fuel Doubled")
                  (Class|GameplayStatics|PlaySoundAttached "/Game/Audio/FuelIncrease.FuelIncrease" _mesh)
                  (goto _label)
                  (else
                    (bind _outactors_4 (Actor|GetAllActorsOfClass "/Game/Blueprints/PickUps/LevelDest.LevelDest_C"))
                    (for _array_element_4 _outactors_4
                      (bind _asleveldest_c (Utilities|Casting|CastToLevelDest _array_element_4))
                      (if (== OtherActor _asleveldest_c)
                        (Game|SpawnActorfromClass "/Game/Blueprints/ArrowPointer.ArrowPointer_C" (Math|Conversions|ToTransform(Vector) (Transformation|GetActorLocation)) false 0)
                        (Development|PrintString "Desination Found")
                        (Class|GameplayStatics|PlaySoundAttached "/Game/Audio/Director.Director" _mesh)
                        (goto _label)
                        (else
                          (bind _outactors_5 (Actor|GetAllActorsOfClass "/Game/Blueprints/PickUps/JumpBoost.JumpBoost_C"))
                          (for _array_element_5 _outactors_5
                            (bind _asjumpboost_c (Utilities|Casting|CastToJumpBoost _array_element_5))
                            (if (== OtherActor _asjumpboost_c)
                              (Variables|Default|SetJumpPower 3.0)
                              (Development|PrintString "Booster Equipped")
                              (Class|GameplayStatics|PlaySoundAttached "/Game/Audio/JumpBoost.JumpBoost" _mesh)
                              (goto _label)
                              (else
                                (bind _outactors_6 (Actor|GetAllActorsOfClass "/Game/Blueprints/PickUps/CheckPoint.CheckPoint_C"))
                                (for _array_element_6 _outactors_6
                                  (bind _ascheckpoint_c (Utilities|Casting|CastToCheckPoint _array_element_6))
                                  (if (== OtherActor _ascheckpoint_c)
                                    (Variables|Default|SetCheckPoint (Transformation|GetActorLocation))
                                    (Development|PrintString "Check Point Established")
                                    (Class|GameplayStatics|PlaySoundAttached "/Game/Audio/SetCheckPoint.SetCheckPoint" _mesh)
                                    (Variables|Default|SetHealth 5)
                                    (goto _label)))
                                (bind _ascheckpoint_c_2 (Utilities|Casting|CastToCheckPoint _array_element_6))
                                (if (== OtherActor _ascheckpoint_c_2)
                                  (Variables|Default|SetCheckPoint (Transformation|GetActorLocation))
                                  (Development|PrintString "Check Point Established")
                                  (Class|GameplayStatics|PlaySoundAttached "/Game/Audio/SetCheckPoint.SetCheckPoint" _mesh)
                                  (Variables|Default|SetHealth 5)
                                  (goto _label)))))
                          (bind _outactors_7 (Actor|GetAllActorsOfClass "/Game/Blueprints/PickUps/CheckPoint.CheckPoint_C"))
                          (for _array_element_7 _outactors_7
                            (bind _ascheckpoint_c_3 (Utilities|Casting|CastToCheckPoint _array_element_7))
                            (if (== OtherActor _ascheckpoint_c_3)
                              (Variables|Default|SetCheckPoint (Transformation|GetActorLocation))
                              (Development|PrintString "Check Point Established")
                              (Class|GameplayStatics|PlaySoundAttached "/Game/Audio/SetCheckPoint.SetCheckPoint" _mesh)
                              (Variables|Default|SetHealth 5)
                              (goto _label)))
                          (bind _ascheckpoint_c_4 (Utilities|Casting|CastToCheckPoint _array_element_7))
                          (if (== OtherActor _ascheckpoint_c_4)
                            (Variables|Default|SetCheckPoint (Transformation|GetActorLocation))
                            (Development|PrintString "Check Point Established")
                            (Class|GameplayStatics|PlaySoundAttached "/Game/Audio/SetCheckPoint.SetCheckPoint" _mesh)
                            (Variables|Default|SetHealth 5)
                            (goto _label)))))
                    (bind _outactors_8 (Actor|GetAllActorsOfClass "/Game/Blueprints/PickUps/JumpBoost.JumpBoost_C"))
                    (for _array_element_8 _outactors_8
                      (bind _asjumpboost_c_2 (Utilities|Casting|CastToJumpBoost _array_element_8))
                      (if (== OtherActor _asjumpboost_c_2)
                        (Variables|Default|SetJumpPower 3.0)
                        (Development|PrintString "Booster Equipped")
                        (Class|GameplayStatics|PlaySoundAttached "/Game/Audio/JumpBoost.JumpBoost" _mesh)
                        (goto _label)
                        (else
                          (bind _outactors_9 (Actor|GetAllActorsOfClass "/Game/Blueprints/PickUps/CheckPoint.CheckPoint_C"))
                          (for _array_element_9 _outactors_9
                            (bind _ascheckpoint_c_5 (Utilities|Casting|CastToCheckPoint _array_element_9))
                            (if (== OtherActor _ascheckpoint_c_5)
                              (Variables|Default|SetCheckPoint (Transformation|GetActorLocation))
                              (Development|PrintString "Check Point Established")
                              (Class|GameplayStatics|PlaySoundAttached "/Game/Audio/SetCheckPoint.SetCheckPoint" _mesh)
                              (Variables|Default|SetHealth 5)
                              (goto _label)))
                          (bind _ascheckpoint_c_6 (Utilities|Casting|CastToCheckPoint _array_element_9))
                          (if (== OtherActor _ascheckpoint_c_6)
                            (Variables|Default|SetCheckPoint (Transformation|GetActorLocation))
                            (Development|PrintString "Check Point Established")
                            (Class|GameplayStatics|PlaySoundAttached "/Game/Audio/SetCheckPoint.SetCheckPoint" _mesh)
                            (Variables|Default|SetHealth 5)
                            (goto _label)))))
                    (bind _outactors_10 (Actor|GetAllActorsOfClass "/Game/Blueprints/PickUps/CheckPoint.CheckPoint_C"))
                    (for _array_element_10 _outactors_10
                      (bind _ascheckpoint_c_7 (Utilities|Casting|CastToCheckPoint _array_element_10))
                      (if (== OtherActor _ascheckpoint_c_7)
                        (Variables|Default|SetCheckPoint (Transformation|GetActorLocation))
                        (Development|PrintString "Check Point Established")
                        (Class|GameplayStatics|PlaySoundAttached "/Game/Audio/SetCheckPoint.SetCheckPoint" _mesh)
                        (Variables|Default|SetHealth 5)
                        (goto _label)))
                    (bind _ascheckpoint_c_8 (Utilities|Casting|CastToCheckPoint _array_element_10))
                    (if (== OtherActor _ascheckpoint_c_8)
                      (Variables|Default|SetCheckPoint (Transformation|GetActorLocation))
                      (Development|PrintString "Check Point Established")
                      (Class|GameplayStatics|PlaySoundAttached "/Game/Audio/SetCheckPoint.SetCheckPoint" _mesh)
                      (Variables|Default|SetHealth 5)
                      (goto _label)))))
              (bind _outactors_11 (Actor|GetAllActorsOfClass "/Game/Blueprints/PickUps/LevelDest.LevelDest_C"))
              (for _array_element_11 _outactors_11
                (bind _asleveldest_c_2 (Utilities|Casting|CastToLevelDest _array_element_11))
                (if (== OtherActor _asleveldest_c_2)
                  (Game|SpawnActorfromClass "/Game/Blueprints/ArrowPointer.ArrowPointer_C" (Math|Conversions|ToTransform(Vector) (Transformation|GetActorLocation)) false 0)
                  (Development|PrintString "Desination Found")
                  (Class|GameplayStatics|PlaySoundAttached "/Game/Audio/Director.Director" _mesh)
                  (goto _label)
                  (else
                    (bind _outactors_12 (Actor|GetAllActorsOfClass "/Game/Blueprints/PickUps/JumpBoost.JumpBoost_C"))
                    (for _array_element_12 _outactors_12
                      (bind _asjumpboost_c_3 (Utilities|Casting|CastToJumpBoost _array_element_12))
                      (if (== OtherActor _asjumpboost_c_3)
                        (Variables|Default|SetJumpPower 3.0)
                        (Development|PrintString "Booster Equipped")
                        (Class|GameplayStatics|PlaySoundAttached "/Game/Audio/JumpBoost.JumpBoost" _mesh)
                        (goto _label)
                        (else
                          (bind _outactors_13 (Actor|GetAllActorsOfClass "/Game/Blueprints/PickUps/CheckPoint.CheckPoint_C"))
                          (for _array_element_13 _outactors_13
                            (bind _ascheckpoint_c_9 (Utilities|Casting|CastToCheckPoint _array_element_13))
                            (if (== OtherActor _ascheckpoint_c_9)
                              (Variables|Default|SetCheckPoint (Transformation|GetActorLocation))
                              (Development|PrintString "Check Point Established")
                              (Class|GameplayStatics|PlaySoundAttached "/Game/Audio/SetCheckPoint.SetCheckPoint" _mesh)
                              (Variables|Default|SetHealth 5)
                              (goto _label)))
                          (bind _ascheckpoint_c_10 (Utilities|Casting|CastToCheckPoint _array_element_13))
                          (if (== OtherActor _ascheckpoint_c_10)
                            (Variables|Default|SetCheckPoint (Transformation|GetActorLocation))
                            (Development|PrintString "Check Point Established")
                            (Class|GameplayStatics|PlaySoundAttached "/Game/Audio/SetCheckPoint.SetCheckPoint" _mesh)
                            (Variables|Default|SetHealth 5)
                            (goto _label)))))
                    (bind _outactors_14 (Actor|GetAllActorsOfClass "/Game/Blueprints/PickUps/CheckPoint.CheckPoint_C"))
                    (for _array_element_14 _outactors_14
                      (bind _ascheckpoint_c_11 (Utilities|Casting|CastToCheckPoint _array_element_14))
                      (if (== OtherActor _ascheckpoint_c_11)
                        (Variables|Default|SetCheckPoint (Transformation|GetActorLocation))
                        (Development|PrintString "Check Point Established")
                        (Class|GameplayStatics|PlaySoundAttached "/Game/Audio/SetCheckPoint.SetCheckPoint" _mesh)
                        (Variables|Default|SetHealth 5)
                        (goto _label)))
                    (bind _ascheckpoint_c_12 (Utilities|Casting|CastToCheckPoint _array_element_14))
                    (if (== OtherActor _ascheckpoint_c_12)
                      (Variables|Default|SetCheckPoint (Transformation|GetActorLocation))
                      (Development|PrintString "Check Point Established")
                      (Class|GameplayStatics|PlaySoundAttached "/Game/Audio/SetCheckPoint.SetCheckPoint" _mesh)
                      (Variables|Default|SetHealth 5)
                      (goto _label)))))
              (bind _outactors_15 (Actor|GetAllActorsOfClass "/Game/Blueprints/PickUps/JumpBoost.JumpBoost_C"))
              (for _array_element_15 _outactors_15
                (bind _asjumpboost_c_4 (Utilities|Casting|CastToJumpBoost _array_element_15))
                (if (== OtherActor _asjumpboost_c_4)
                  (Variables|Default|SetJumpPower 3.0)
                  (Development|PrintString "Booster Equipped")
                  (Class|GameplayStatics|PlaySoundAttached "/Game/Audio/JumpBoost.JumpBoost" _mesh)
                  (goto _label)
                  (else
                    (bind _outactors_16 (Actor|GetAllActorsOfClass "/Game/Blueprints/PickUps/CheckPoint.CheckPoint_C"))
                    (for _array_element_16 _outactors_16
                      (bind _ascheckpoint_c_13 (Utilities|Casting|CastToCheckPoint _array_element_16))
                      (if (== OtherActor _ascheckpoint_c_13)
                        (Variables|Default|SetCheckPoint (Transformation|GetActorLocation))
                        (Development|PrintString "Check Point Established")
                        (Class|GameplayStatics|PlaySoundAttached "/Game/Audio/SetCheckPoint.SetCheckPoint" _mesh)
                        (Variables|Default|SetHealth 5)
                        (goto _label)))
                    (bind _ascheckpoint_c_14 (Utilities|Casting|CastToCheckPoint _array_element_16))
                    (if (== OtherActor _ascheckpoint_c_14)
                      (Variables|Default|SetCheckPoint (Transformation|GetActorLocation))
                      (Development|PrintString "Check Point Established")
                      (Class|GameplayStatics|PlaySoundAttached "/Game/Audio/SetCheckPoint.SetCheckPoint" _mesh)
                      (Variables|Default|SetHealth 5)
                      (goto _label)))))
              (bind _outactors_17 (Actor|GetAllActorsOfClass "/Game/Blueprints/PickUps/CheckPoint.CheckPoint_C"))
              (for _array_element_17 _outactors_17
                (bind _ascheckpoint_c_15 (Utilities|Casting|CastToCheckPoint _array_element_17))
                (if (== OtherActor _ascheckpoint_c_15)
                  (Variables|Default|SetCheckPoint (Transformation|GetActorLocation))
                  (Development|PrintString "Check Point Established")
                  (Class|GameplayStatics|PlaySoundAttached "/Game/Audio/SetCheckPoint.SetCheckPoint" _mesh)
                  (Variables|Default|SetHealth 5)
                  (goto _label)))
              (bind _ascheckpoint_c_16 (Utilities|Casting|CastToCheckPoint _array_element_17))
              (if (== OtherActor _ascheckpoint_c_16)
                (Variables|Default|SetCheckPoint (Transformation|GetActorLocation))
                (Development|PrintString "Check Point Established")
                (Class|GameplayStatics|PlaySoundAttached "/Game/Audio/SetCheckPoint.SetCheckPoint" _mesh)
                (Variables|Default|SetHealth 5)
                (goto _label)))))
        (bind _outactors_18 (Actor|GetAllActorsOfClass "/Game/Blueprints/PickUps/FuelExpansion.FuelExpansion_C"))
        (for _array_element_18 _outactors_18
          (bind _asfuelexpansion_c_2 (Utilities|Casting|CastToFuelExpansion _array_element_18))
          (if (== OtherActor _asfuelexpansion_c_2)
            (Variables|Default|SetMaxFuel 199)
            (Variables|Default|SetFuel (Variables|Default|GetMaxFuel))
            (Development|PrintString "Jet Pack Fuel Doubled")
            (Class|GameplayStatics|PlaySoundAttached "/Game/Audio/FuelIncrease.FuelIncrease" _mesh)
            (goto _label)
            (else
              (bind _outactors_19 (Actor|GetAllActorsOfClass "/Game/Blueprints/PickUps/LevelDest.LevelDest_C"))
              (for _array_element_19 _outactors_19
                (bind _asleveldest_c_3 (Utilities|Casting|CastToLevelDest _array_element_19))
                (if (== OtherActor _asleveldest_c_3)
                  (Game|SpawnActorfromClass "/Game/Blueprints/ArrowPointer.ArrowPointer_C" (Math|Conversions|ToTransform(Vector) (Transformation|GetActorLocation)) false 0)
                  (Development|PrintString "Desination Found")
                  (Class|GameplayStatics|PlaySoundAttached "/Game/Audio/Director.Director" _mesh)
                  (goto _label)
                  (else
                    (bind _outactors_20 (Actor|GetAllActorsOfClass "/Game/Blueprints/PickUps/JumpBoost.JumpBoost_C"))
                    (for _array_element_20 _outactors_20
                      (bind _asjumpboost_c_5 (Utilities|Casting|CastToJumpBoost _array_element_20))
                      (if (== OtherActor _asjumpboost_c_5)
                        (Variables|Default|SetJumpPower 3.0)
                        (Development|PrintString "Booster Equipped")
                        (Class|GameplayStatics|PlaySoundAttached "/Game/Audio/JumpBoost.JumpBoost" _mesh)
                        (goto _label)
                        (else
                          (bind _outactors_21 (Actor|GetAllActorsOfClass "/Game/Blueprints/PickUps/CheckPoint.CheckPoint_C"))
                          (for _array_element_21 _outactors_21
                            (bind _ascheckpoint_c_17 (Utilities|Casting|CastToCheckPoint _array_element_21))
                            (if (== OtherActor _ascheckpoint_c_17)
                              (Variables|Default|SetCheckPoint (Transformation|GetActorLocation))
                              (Development|PrintString "Check Point Established")
                              (Class|GameplayStatics|PlaySoundAttached "/Game/Audio/SetCheckPoint.SetCheckPoint" _mesh)
                              (Variables|Default|SetHealth 5)
                              (goto _label)))
                          (bind _ascheckpoint_c_18 (Utilities|Casting|CastToCheckPoint _array_element_21))
                          (if (== OtherActor _ascheckpoint_c_18)
                            (Variables|Default|SetCheckPoint (Transformation|GetActorLocation))
                            (Development|PrintString "Check Point Established")
                            (Class|GameplayStatics|PlaySoundAttached "/Game/Audio/SetCheckPoint.SetCheckPoint" _mesh)
                            (Variables|Default|SetHealth 5)
                            (goto _label)))))
                    (bind _outactors_22 (Actor|GetAllActorsOfClass "/Game/Blueprints/PickUps/CheckPoint.CheckPoint_C"))
                    (for _array_element_22 _outactors_22
                      (bind _ascheckpoint_c_19 (Utilities|Casting|CastToCheckPoint _array_element_22))
                      (if (== OtherActor _ascheckpoint_c_19)
                        (Variables|Default|SetCheckPoint (Transformation|GetActorLocation))
                        (Development|PrintString "Check Point Established")
                        (Class|GameplayStatics|PlaySoundAttached "/Game/Audio/SetCheckPoint.SetCheckPoint" _mesh)
                        (Variables|Default|SetHealth 5)
                        (goto _label)))
                    (bind _ascheckpoint_c_20 (Utilities|Casting|CastToCheckPoint _array_element_22))
                    (if (== OtherActor _ascheckpoint_c_20)
                      (Variables|Default|SetCheckPoint (Transformation|GetActorLocation))
                      (Development|PrintString "Check Point Established")
                      (Class|GameplayStatics|PlaySoundAttached "/Game/Audio/SetCheckPoint.SetCheckPoint" _mesh)
                      (Variables|Default|SetHealth 5)
                      (goto _label)))))
              (bind _outactors_23 (Actor|GetAllActorsOfClass "/Game/Blueprints/PickUps/JumpBoost.JumpBoost_C"))
              (for _array_element_23 _outactors_23
                (bind _asjumpboost_c_6 (Utilities|Casting|CastToJumpBoost _array_element_23))
                (if (== OtherActor _asjumpboost_c_6)
                  (Variables|Default|SetJumpPower 3.0)
                  (Development|PrintString "Booster Equipped")
                  (Class|GameplayStatics|PlaySoundAttached "/Game/Audio/JumpBoost.JumpBoost" _mesh)
                  (goto _label)
                  (else
                    (bind _outactors_24 (Actor|GetAllActorsOfClass "/Game/Blueprints/PickUps/CheckPoint.CheckPoint_C"))
                    (for _array_element_24 _outactors_24
                      (bind _ascheckpoint_c_21 (Utilities|Casting|CastToCheckPoint _array_element_24))
                      (if (== OtherActor _ascheckpoint_c_21)
                        (Variables|Default|SetCheckPoint (Transformation|GetActorLocation))
                        (Development|PrintString "Check Point Established")
                        (Class|GameplayStatics|PlaySoundAttached "/Game/Audio/SetCheckPoint.SetCheckPoint" _mesh)
                        (Variables|Default|SetHealth 5)
                        (goto _label)))
                    (bind _ascheckpoint_c_22 (Utilities|Casting|CastToCheckPoint _array_element_24))
                    (if (== OtherActor _ascheckpoint_c_22)
                      (Variables|Default|SetCheckPoint (Transformation|GetActorLocation))
                      (Development|PrintString "Check Point Established")
                      (Class|GameplayStatics|PlaySoundAttached "/Game/Audio/SetCheckPoint.SetCheckPoint" _mesh)
                      (Variables|Default|SetHealth 5)
                      (goto _label)))))
              (bind _outactors_25 (Actor|GetAllActorsOfClass "/Game/Blueprints/PickUps/CheckPoint.CheckPoint_C"))
              (for _array_element_25 _outactors_25
                (bind _ascheckpoint_c_23 (Utilities|Casting|CastToCheckPoint _array_element_25))
                (if (== OtherActor _ascheckpoint_c_23)
                  (Variables|Default|SetCheckPoint (Transformation|GetActorLocation))
                  (Development|PrintString "Check Point Established")
                  (Class|GameplayStatics|PlaySoundAttached "/Game/Audio/SetCheckPoint.SetCheckPoint" _mesh)
                  (Variables|Default|SetHealth 5)
                  (goto _label)))
              (bind _ascheckpoint_c_24 (Utilities|Casting|CastToCheckPoint _array_element_25))
              (if (== OtherActor _ascheckpoint_c_24)
                (Variables|Default|SetCheckPoint (Transformation|GetActorLocation))
                (Development|PrintString "Check Point Established")
                (Class|GameplayStatics|PlaySoundAttached "/Game/Audio/SetCheckPoint.SetCheckPoint" _mesh)
                (Variables|Default|SetHealth 5)
                (goto _label)))))
        (bind _outactors_26 (Actor|GetAllActorsOfClass "/Game/Blueprints/PickUps/LevelDest.LevelDest_C"))
        (for _array_element_26 _outactors_26
          (bind _asleveldest_c_4 (Utilities|Casting|CastToLevelDest _array_element_26))
          (if (== OtherActor _asleveldest_c_4)
            (Game|SpawnActorfromClass "/Game/Blueprints/ArrowPointer.ArrowPointer_C" (Math|Conversions|ToTransform(Vector) (Transformation|GetActorLocation)) false 0)
            (Development|PrintString "Desination Found")
            (Class|GameplayStatics|PlaySoundAttached "/Game/Audio/Director.Director" _mesh)
            (goto _label)
            (else
              (bind _outactors_27 (Actor|GetAllActorsOfClass "/Game/Blueprints/PickUps/JumpBoost.JumpBoost_C"))
              (for _array_element_27 _outactors_27
                (bind _asjumpboost_c_7 (Utilities|Casting|CastToJumpBoost _array_element_27))
                (if (== OtherActor _asjumpboost_c_7)
                  (Variables|Default|SetJumpPower 3.0)
                  (Development|PrintString "Booster Equipped")
                  (Class|GameplayStatics|PlaySoundAttached "/Game/Audio/JumpBoost.JumpBoost" _mesh)
                  (goto _label)
                  (else
                    (bind _outactors_28 (Actor|GetAllActorsOfClass "/Game/Blueprints/PickUps/CheckPoint.CheckPoint_C"))
                    (for _array_element_28 _outactors_28
                      (bind _ascheckpoint_c_25 (Utilities|Casting|CastToCheckPoint _array_element_28))
                      (if (== OtherActor _ascheckpoint_c_25)
                        (Variables|Default|SetCheckPoint (Transformation|GetActorLocation))
                        (Development|PrintString "Check Point Established")
                        (Class|GameplayStatics|PlaySoundAttached "/Game/Audio/SetCheckPoint.SetCheckPoint" _mesh)
                        (Variables|Default|SetHealth 5)
                        (goto _label)))
                    (bind _ascheckpoint_c_26 (Utilities|Casting|CastToCheckPoint _array_element_28))
                    (if (== OtherActor _ascheckpoint_c_26)
                      (Variables|Default|SetCheckPoint (Transformation|GetActorLocation))
                      (Development|PrintString "Check Point Established")
                      (Class|GameplayStatics|PlaySoundAttached "/Game/Audio/SetCheckPoint.SetCheckPoint" _mesh)
                      (Variables|Default|SetHealth 5)
                      (goto _label)))))
              (bind _outactors_29 (Actor|GetAllActorsOfClass "/Game/Blueprints/PickUps/CheckPoint.CheckPoint_C"))
              (for _array_element_29 _outactors_29
                (bind _ascheckpoint_c_27 (Utilities|Casting|CastToCheckPoint _array_element_29))
                (if (== OtherActor _ascheckpoint_c_27)
                  (Variables|Default|SetCheckPoint (Transformation|GetActorLocation))
                  (Development|PrintString "Check Point Established")
                  (Class|GameplayStatics|PlaySoundAttached "/Game/Audio/SetCheckPoint.SetCheckPoint" _mesh)
                  (Variables|Default|SetHealth 5)
                  (goto _label)))
              (bind _ascheckpoint_c_28 (Utilities|Casting|CastToCheckPoint _array_element_29))
              (if (== OtherActor _ascheckpoint_c_28)
                (Variables|Default|SetCheckPoint (Transformation|GetActorLocation))
                (Development|PrintString "Check Point Established")
                (Class|GameplayStatics|PlaySoundAttached "/Game/Audio/SetCheckPoint.SetCheckPoint" _mesh)
                (Variables|Default|SetHealth 5)
                (goto _label)))))
        (bind _outactors_30 (Actor|GetAllActorsOfClass "/Game/Blueprints/PickUps/JumpBoost.JumpBoost_C"))
        (for _array_element_30 _outactors_30
          (bind _asjumpboost_c_8 (Utilities|Casting|CastToJumpBoost _array_element_30))
          (if (== OtherActor _asjumpboost_c_8)
            (Variables|Default|SetJumpPower 3.0)
            (Development|PrintString "Booster Equipped")
            (Class|GameplayStatics|PlaySoundAttached "/Game/Audio/JumpBoost.JumpBoost" _mesh)
            (goto _label)
            (else
              (bind _outactors_31 (Actor|GetAllActorsOfClass "/Game/Blueprints/PickUps/CheckPoint.CheckPoint_C"))
              (for _array_element_31 _outactors_31
                (bind _ascheckpoint_c_29 (Utilities|Casting|CastToCheckPoint _array_element_31))
                (if (== OtherActor _ascheckpoint_c_29)
                  (Variables|Default|SetCheckPoint (Transformation|GetActorLocation))
                  (Development|PrintString "Check Point Established")
                  (Class|GameplayStatics|PlaySoundAttached "/Game/Audio/SetCheckPoint.SetCheckPoint" _mesh)
                  (Variables|Default|SetHealth 5)
                  (goto _label)))
              (bind _ascheckpoint_c_30 (Utilities|Casting|CastToCheckPoint _array_element_31))
              (if (== OtherActor _ascheckpoint_c_30)
                (Variables|Default|SetCheckPoint (Transformation|GetActorLocation))
                (Development|PrintString "Check Point Established")
                (Class|GameplayStatics|PlaySoundAttached "/Game/Audio/SetCheckPoint.SetCheckPoint" _mesh)
                (Variables|Default|SetHealth 5)
                (goto _label)))))
        (bind _outactors_32 (Actor|GetAllActorsOfClass "/Game/Blueprints/PickUps/CheckPoint.CheckPoint_C"))
        (for _array_element_32 _outactors_32
          (bind _ascheckpoint_c_31 (Utilities|Casting|CastToCheckPoint _array_element_32))
          (if (== OtherActor _ascheckpoint_c_31)
            (Variables|Default|SetCheckPoint (Transformation|GetActorLocation))
            (Development|PrintString "Check Point Established")
            (Class|GameplayStatics|PlaySoundAttached "/Game/Audio/SetCheckPoint.SetCheckPoint" _mesh)
            (Variables|Default|SetHealth 5)
            (goto _label)))
        (bind _ascheckpoint_c_32 (Utilities|Casting|CastToCheckPoint _array_element_32))
        (if (== OtherActor _ascheckpoint_c_32)
          (Variables|Default|SetCheckPoint (Transformation|GetActorLocation))
          (Development|PrintString "Check Point Established")
          (Class|GameplayStatics|PlaySoundAttached "/Game/Audio/SetCheckPoint.SetCheckPoint" _mesh)
          (Variables|Default|SetHealth 5)
          (goto _label)))))
  (bind _outactors_33 (Actor|GetAllActorsOfClass "/Game/Blueprints/PickUps/AirRefuel.AirRefuel_C"))
  (for _array_element_33 _outactors_33
    (bind _asairrefuel_c_2 (Utilities|Casting|CastToAirRefuel _array_element_33))
    (if (== OtherActor _asairrefuel_c_2)
      (Variables|Default|SetAirRefuel true)
      (Development|PrintString "Air Refuel Enabled")
      (Class|GameplayStatics|PlaySoundAttached "/Game/Audio/AirRefueler.AirRefueler" _mesh)
      (Actor|DestroyActor OtherActor :!label _label_2)
      (else
        (bind _outactors_34 (Actor|GetAllActorsOfClass "/Game/Blueprints/PickUps/FuelExpansion.FuelExpansion_C"))
        (for _array_element_34 _outactors_34
          (bind _asfuelexpansion_c_3 (Utilities|Casting|CastToFuelExpansion _array_element_34))
          (if (== OtherActor _asfuelexpansion_c_3)
            (Variables|Default|SetMaxFuel 199)
            (Variables|Default|SetFuel (Variables|Default|GetMaxFuel))
            (Development|PrintString "Jet Pack Fuel Doubled")
            (Class|GameplayStatics|PlaySoundAttached "/Game/Audio/FuelIncrease.FuelIncrease" _mesh)
            (goto _label_2)
            (else
              (bind _outactors_35 (Actor|GetAllActorsOfClass "/Game/Blueprints/PickUps/LevelDest.LevelDest_C"))
              (for _array_element_35 _outactors_35
                (bind _asleveldest_c_5 (Utilities|Casting|CastToLevelDest _array_element_35))
                (if (== OtherActor _asleveldest_c_5)
                  (Game|SpawnActorfromClass "/Game/Blueprints/ArrowPointer.ArrowPointer_C" (Math|Conversions|ToTransform(Vector) (Transformation|GetActorLocation)) false 0)
                  (Development|PrintString "Desination Found")
                  (Class|GameplayStatics|PlaySoundAttached "/Game/Audio/Director.Director" _mesh)
                  (goto _label_2)
                  (else
                    (bind _outactors_36 (Actor|GetAllActorsOfClass "/Game/Blueprints/PickUps/JumpBoost.JumpBoost_C"))
                    (for _array_element_36 _outactors_36
                      (bind _asjumpboost_c_9 (Utilities|Casting|CastToJumpBoost _array_element_36))
                      (if (== OtherActor _asjumpboost_c_9)
                        (Variables|Default|SetJumpPower 3.0)
                        (Development|PrintString "Booster Equipped")
                        (Class|GameplayStatics|PlaySoundAttached "/Game/Audio/JumpBoost.JumpBoost" _mesh)
                        (goto _label_2)
                        (else
                          (bind _outactors_37 (Actor|GetAllActorsOfClass "/Game/Blueprints/PickUps/CheckPoint.CheckPoint_C"))
                          (for _array_element_37 _outactors_37
                            (bind _ascheckpoint_c_33 (Utilities|Casting|CastToCheckPoint _array_element_37))
                            (if (== OtherActor _ascheckpoint_c_33)
                              (Variables|Default|SetCheckPoint (Transformation|GetActorLocation))
                              (Development|PrintString "Check Point Established")
                              (Class|GameplayStatics|PlaySoundAttached "/Game/Audio/SetCheckPoint.SetCheckPoint" _mesh)
                              (Variables|Default|SetHealth 5)
                              (goto _label_2)))
                          (bind _ascheckpoint_c_34 (Utilities|Casting|CastToCheckPoint _array_element_37))
                          (if (== OtherActor _ascheckpoint_c_34)
                            (Variables|Default|SetCheckPoint (Transformation|GetActorLocation))
                            (Development|PrintString "Check Point Established")
                            (Class|GameplayStatics|PlaySoundAttached "/Game/Audio/SetCheckPoint.SetCheckPoint" _mesh)
                            (Variables|Default|SetHealth 5)
                            (goto _label_2)))))
                    (bind _outactors_38 (Actor|GetAllActorsOfClass "/Game/Blueprints/PickUps/CheckPoint.CheckPoint_C"))
                    (for _array_element_38 _outactors_38
                      (bind _ascheckpoint_c_35 (Utilities|Casting|CastToCheckPoint _array_element_38))
                      (if (== OtherActor _ascheckpoint_c_35)
                        (Variables|Default|SetCheckPoint (Transformation|GetActorLocation))
                        (Development|PrintString "Check Point Established")
                        (Class|GameplayStatics|PlaySoundAttached "/Game/Audio/SetCheckPoint.SetCheckPoint" _mesh)
                        (Variables|Default|SetHealth 5)
                        (goto _label_2)))
                    (bind _ascheckpoint_c_36 (Utilities|Casting|CastToCheckPoint _array_element_38))
                    (if (== OtherActor _ascheckpoint_c_36)
                      (Variables|Default|SetCheckPoint (Transformation|GetActorLocation))
                      (Development|PrintString "Check Point Established")
                      (Class|GameplayStatics|PlaySoundAttached "/Game/Audio/SetCheckPoint.SetCheckPoint" _mesh)
                      (Variables|Default|SetHealth 5)
                      (goto _label_2)))))
              (bind _outactors_39 (Actor|GetAllActorsOfClass "/Game/Blueprints/PickUps/JumpBoost.JumpBoost_C"))
              (for _array_element_39 _outactors_39
                (bind _asjumpboost_c_10 (Utilities|Casting|CastToJumpBoost _array_element_39))
                (if (== OtherActor _asjumpboost_c_10)
                  (Variables|Default|SetJumpPower 3.0)
                  (Development|PrintString "Booster Equipped")
                  (Class|GameplayStatics|PlaySoundAttached "/Game/Audio/JumpBoost.JumpBoost" _mesh)
                  (goto _label_2)
                  (else
                    (bind _outactors_40 (Actor|GetAllActorsOfClass "/Game/Blueprints/PickUps/CheckPoint.CheckPoint_C"))
                    (for _array_element_40 _outactors_40
                      (bind _ascheckpoint_c_37 (Utilities|Casting|CastToCheckPoint _array_element_40))
                      (if (== OtherActor _ascheckpoint_c_37)
                        (Variables|Default|SetCheckPoint (Transformation|GetActorLocation))
                        (Development|PrintString "Check Point Established")
                        (Class|GameplayStatics|PlaySoundAttached "/Game/Audio/SetCheckPoint.SetCheckPoint" _mesh)
                        (Variables|Default|SetHealth 5)
                        (goto _label_2)))
                    (bind _ascheckpoint_c_38 (Utilities|Casting|CastToCheckPoint _array_element_40))
                    (if (== OtherActor _ascheckpoint_c_38)
                      (Variables|Default|SetCheckPoint (Transformation|GetActorLocation))
                      (Development|PrintString "Check Point Established")
                      (Class|GameplayStatics|PlaySoundAttached "/Game/Audio/SetCheckPoint.SetCheckPoint" _mesh)
                      (Variables|Default|SetHealth 5)
                      (goto _label_2)))))
              (bind _outactors_41 (Actor|GetAllActorsOfClass "/Game/Blueprints/PickUps/CheckPoint.CheckPoint_C"))
              (for _array_element_41 _outactors_41
                (bind _ascheckpoint_c_39 (Utilities|Casting|CastToCheckPoint _array_element_41))
                (if (== OtherActor _ascheckpoint_c_39)
                  (Variables|Default|SetCheckPoint (Transformation|GetActorLocation))
                  (Development|PrintString "Check Point Established")
                  (Class|GameplayStatics|PlaySoundAttached "/Game/Audio/SetCheckPoint.SetCheckPoint" _mesh)
                  (Variables|Default|SetHealth 5)
                  (goto _label_2)))
              (bind _ascheckpoint_c_40 (Utilities|Casting|CastToCheckPoint _array_element_41))
              (if (== OtherActor _ascheckpoint_c_40)
                (Variables|Default|SetCheckPoint (Transformation|GetActorLocation))
                (Development|PrintString "Check Point Established")
                (Class|GameplayStatics|PlaySoundAttached "/Game/Audio/SetCheckPoint.SetCheckPoint" _mesh)
                (Variables|Default|SetHealth 5)
                (goto _label_2)))))
        (bind _outactors_42 (Actor|GetAllActorsOfClass "/Game/Blueprints/PickUps/LevelDest.LevelDest_C"))
        (for _array_element_42 _outactors_42
          (bind _asleveldest_c_6 (Utilities|Casting|CastToLevelDest _array_element_42))
          (if (== OtherActor _asleveldest_c_6)
            (Game|SpawnActorfromClass "/Game/Blueprints/ArrowPointer.ArrowPointer_C" (Math|Conversions|ToTransform(Vector) (Transformation|GetActorLocation)) false 0)
            (Development|PrintString "Desination Found")
            (Class|GameplayStatics|PlaySoundAttached "/Game/Audio/Director.Director" _mesh)
            (goto _label_2)
            (else
              (bind _outactors_43 (Actor|GetAllActorsOfClass "/Game/Blueprints/PickUps/JumpBoost.JumpBoost_C"))
              (for _array_element_43 _outactors_43
                (bind _asjumpboost_c_11 (Utilities|Casting|CastToJumpBoost _array_element_43))
                (if (== OtherActor _asjumpboost_c_11)
                  (Variables|Default|SetJumpPower 3.0)
                  (Development|PrintString "Booster Equipped")
                  (Class|GameplayStatics|PlaySoundAttached "/Game/Audio/JumpBoost.JumpBoost" _mesh)
                  (goto _label_2)
                  (else
                    (bind _outactors_44 (Actor|GetAllActorsOfClass "/Game/Blueprints/PickUps/CheckPoint.CheckPoint_C"))
                    (for _array_element_44 _outactors_44
                      (bind _ascheckpoint_c_41 (Utilities|Casting|CastToCheckPoint _array_element_44))
                      (if (== OtherActor _ascheckpoint_c_41)
                        (Variables|Default|SetCheckPoint (Transformation|GetActorLocation))
                        (Development|PrintString "Check Point Established")
                        (Class|GameplayStatics|PlaySoundAttached "/Game/Audio/SetCheckPoint.SetCheckPoint" _mesh)
                        (Variables|Default|SetHealth 5)
                        (goto _label_2)))
                    (bind _ascheckpoint_c_42 (Utilities|Casting|CastToCheckPoint _array_element_44))
                    (if (== OtherActor _ascheckpoint_c_42)
                      (Variables|Default|SetCheckPoint (Transformation|GetActorLocation))
                      (Development|PrintString "Check Point Established")
                      (Class|GameplayStatics|PlaySoundAttached "/Game/Audio/SetCheckPoint.SetCheckPoint" _mesh)
                      (Variables|Default|SetHealth 5)
                      (goto _label_2)))))
              (bind _outactors_45 (Actor|GetAllActorsOfClass "/Game/Blueprints/PickUps/CheckPoint.CheckPoint_C"))
              (for _array_element_45 _outactors_45
                (bind _ascheckpoint_c_43 (Utilities|Casting|CastToCheckPoint _array_element_45))
                (if (== OtherActor _ascheckpoint_c_43)
                  (Variables|Default|SetCheckPoint (Transformation|GetActorLocation))
                  (Development|PrintString "Check Point Established")
                  (Class|GameplayStatics|PlaySoundAttached "/Game/Audio/SetCheckPoint.SetCheckPoint" _mesh)
                  (Variables|Default|SetHealth 5)
                  (goto _label_2)))
              (bind _ascheckpoint_c_44 (Utilities|Casting|CastToCheckPoint _array_element_45))
              (if (== OtherActor _ascheckpoint_c_44)
                (Variables|Default|SetCheckPoint (Transformation|GetActorLocation))
                (Development|PrintString "Check Point Established")
                (Class|GameplayStatics|PlaySoundAttached "/Game/Audio/SetCheckPoint.SetCheckPoint" _mesh)
                (Variables|Default|SetHealth 5)
                (goto _label_2)))))
        (bind _outactors_46 (Actor|GetAllActorsOfClass "/Game/Blueprints/PickUps/JumpBoost.JumpBoost_C"))
        (for _array_element_46 _outactors_46
          (bind _asjumpboost_c_12 (Utilities|Casting|CastToJumpBoost _array_element_46))
          (if (== OtherActor _asjumpboost_c_12)
            (Variables|Default|SetJumpPower 3.0)
            (Development|PrintString "Booster Equipped")
            (Class|GameplayStatics|PlaySoundAttached "/Game/Audio/JumpBoost.JumpBoost" _mesh)
            (goto _label_2)
            (else
              (bind _outactors_47 (Actor|GetAllActorsOfClass "/Game/Blueprints/PickUps/CheckPoint.CheckPoint_C"))
              (for _array_element_47 _outactors_47
                (bind _ascheckpoint_c_45 (Utilities|Casting|CastToCheckPoint _array_element_47))
                (if (== OtherActor _ascheckpoint_c_45)
                  (Variables|Default|SetCheckPoint (Transformation|GetActorLocation))
                  (Development|PrintString "Check Point Established")
                  (Class|GameplayStatics|PlaySoundAttached "/Game/Audio/SetCheckPoint.SetCheckPoint" _mesh)
                  (Variables|Default|SetHealth 5)
                  (goto _label_2)))
              (bind _ascheckpoint_c_46 (Utilities|Casting|CastToCheckPoint _array_element_47))
              (if (== OtherActor _ascheckpoint_c_46)
                (Variables|Default|SetCheckPoint (Transformation|GetActorLocation))
                (Development|PrintString "Check Point Established")
                (Class|GameplayStatics|PlaySoundAttached "/Game/Audio/SetCheckPoint.SetCheckPoint" _mesh)
                (Variables|Default|SetHealth 5)
                (goto _label_2)))))
        (bind _outactors_48 (Actor|GetAllActorsOfClass "/Game/Blueprints/PickUps/CheckPoint.CheckPoint_C"))
        (for _array_element_48 _outactors_48
          (bind _ascheckpoint_c_47 (Utilities|Casting|CastToCheckPoint _array_element_48))
          (if (== OtherActor _ascheckpoint_c_47)
            (Variables|Default|SetCheckPoint (Transformation|GetActorLocation))
            (Development|PrintString "Check Point Established")
            (Class|GameplayStatics|PlaySoundAttached "/Game/Audio/SetCheckPoint.SetCheckPoint" _mesh)
            (Variables|Default|SetHealth 5)
            (goto _label_2)))
        (bind _ascheckpoint_c_48 (Utilities|Casting|CastToCheckPoint _array_element_48))
        (if (== OtherActor _ascheckpoint_c_48)
          (Variables|Default|SetCheckPoint (Transformation|GetActorLocation))
          (Development|PrintString "Check Point Established")
          (Class|GameplayStatics|PlaySoundAttached "/Game/Audio/SetCheckPoint.SetCheckPoint" _mesh)
          (Variables|Default|SetHealth 5)
          (goto _label_2)))))
  (bind _outactors_49 (Actor|GetAllActorsOfClass "/Game/Blueprints/PickUps/FuelExpansion.FuelExpansion_C"))
  (for _array_element_49 _outactors_49
    (bind _asfuelexpansion_c_4 (Utilities|Casting|CastToFuelExpansion _array_element_49))
    (if (== OtherActor _asfuelexpansion_c_4)
      (Variables|Default|SetMaxFuel 199)
      (Variables|Default|SetFuel (Variables|Default|GetMaxFuel))
      (Development|PrintString "Jet Pack Fuel Doubled")
      (Class|GameplayStatics|PlaySoundAttached "/Game/Audio/FuelIncrease.FuelIncrease" _mesh)
      (Actor|DestroyActor OtherActor :!label _label_3)
      (else
        (bind _outactors_50 (Actor|GetAllActorsOfClass "/Game/Blueprints/PickUps/LevelDest.LevelDest_C"))
        (for _array_element_50 _outactors_50
          (bind _asleveldest_c_7 (Utilities|Casting|CastToLevelDest _array_element_50))
          (if (== OtherActor _asleveldest_c_7)
            (Game|SpawnActorfromClass "/Game/Blueprints/ArrowPointer.ArrowPointer_C" (Math|Conversions|ToTransform(Vector) (Transformation|GetActorLocation)) false 0)
            (Development|PrintString "Desination Found")
            (Class|GameplayStatics|PlaySoundAttached "/Game/Audio/Director.Director" _mesh)
            (goto _label_3)
            (else
              (bind _outactors_51 (Actor|GetAllActorsOfClass "/Game/Blueprints/PickUps/JumpBoost.JumpBoost_C"))
              (for _array_element_51 _outactors_51
                (bind _asjumpboost_c_13 (Utilities|Casting|CastToJumpBoost _array_element_51))
                (if (== OtherActor _asjumpboost_c_13)
                  (Variables|Default|SetJumpPower 3.0)
                  (Development|PrintString "Booster Equipped")
                  (Class|GameplayStatics|PlaySoundAttached "/Game/Audio/JumpBoost.JumpBoost" _mesh)
                  (goto _label_3)
                  (else
                    (bind _outactors_52 (Actor|GetAllActorsOfClass "/Game/Blueprints/PickUps/CheckPoint.CheckPoint_C"))
                    (for _array_element_52 _outactors_52
                      (bind _ascheckpoint_c_49 (Utilities|Casting|CastToCheckPoint _array_element_52))
                      (if (== OtherActor _ascheckpoint_c_49)
                        (Variables|Default|SetCheckPoint (Transformation|GetActorLocation))
                        (Development|PrintString "Check Point Established")
                        (Class|GameplayStatics|PlaySoundAttached "/Game/Audio/SetCheckPoint.SetCheckPoint" _mesh)
                        (Variables|Default|SetHealth 5)
                        (goto _label_3)))
                    (bind _ascheckpoint_c_50 (Utilities|Casting|CastToCheckPoint _array_element_52))
                    (if (== OtherActor _ascheckpoint_c_50)
                      (Variables|Default|SetCheckPoint (Transformation|GetActorLocation))
                      (Development|PrintString "Check Point Established")
                      (Class|GameplayStatics|PlaySoundAttached "/Game/Audio/SetCheckPoint.SetCheckPoint" _mesh)
                      (Variables|Default|SetHealth 5)
                      (goto _label_3)))))
              (bind _outactors_53 (Actor|GetAllActorsOfClass "/Game/Blueprints/PickUps/CheckPoint.CheckPoint_C"))
              (for _array_element_53 _outactors_53
                (bind _ascheckpoint_c_51 (Utilities|Casting|CastToCheckPoint _array_element_53))
                (if (== OtherActor _ascheckpoint_c_51)
                  (Variables|Default|SetCheckPoint (Transformation|GetActorLocation))
                  (Development|PrintString "Check Point Established")
                  (Class|GameplayStatics|PlaySoundAttached "/Game/Audio/SetCheckPoint.SetCheckPoint" _mesh)
                  (Variables|Default|SetHealth 5)
                  (goto _label_3)))
              (bind _ascheckpoint_c_52 (Utilities|Casting|CastToCheckPoint _array_element_53))
              (if (== OtherActor _ascheckpoint_c_52)
                (Variables|Default|SetCheckPoint (Transformation|GetActorLocation))
                (Development|PrintString "Check Point Established")
                (Class|GameplayStatics|PlaySoundAttached "/Game/Audio/SetCheckPoint.SetCheckPoint" _mesh)
                (Variables|Default|SetHealth 5)
                (goto _label_3)))))
        (bind _outactors_54 (Actor|GetAllActorsOfClass "/Game/Blueprints/PickUps/JumpBoost.JumpBoost_C"))
        (for _array_element_54 _outactors_54
          (bind _asjumpboost_c_14 (Utilities|Casting|CastToJumpBoost _array_element_54))
          (if (== OtherActor _asjumpboost_c_14)
            (Variables|Default|SetJumpPower 3.0)
            (Development|PrintString "Booster Equipped")
            (Class|GameplayStatics|PlaySoundAttached "/Game/Audio/JumpBoost.JumpBoost" _mesh)
            (goto _label_3)
            (else
              (bind _outactors_55 (Actor|GetAllActorsOfClass "/Game/Blueprints/PickUps/CheckPoint.CheckPoint_C"))
              (for _array_element_55 _outactors_55
                (bind _ascheckpoint_c_53 (Utilities|Casting|CastToCheckPoint _array_element_55))
                (if (== OtherActor _ascheckpoint_c_53)
                  (Variables|Default|SetCheckPoint (Transformation|GetActorLocation))
                  (Development|PrintString "Check Point Established")
                  (Class|GameplayStatics|PlaySoundAttached "/Game/Audio/SetCheckPoint.SetCheckPoint" _mesh)
                  (Variables|Default|SetHealth 5)
                  (goto _label_3)))
              (bind _ascheckpoint_c_54 (Utilities|Casting|CastToCheckPoint _array_element_55))
              (if (== OtherActor _ascheckpoint_c_54)
                (Variables|Default|SetCheckPoint (Transformation|GetActorLocation))
                (Development|PrintString "Check Point Established")
                (Class|GameplayStatics|PlaySoundAttached "/Game/Audio/SetCheckPoint.SetCheckPoint" _mesh)
                (Variables|Default|SetHealth 5)
                (goto _label_3)))))
        (bind _outactors_56 (Actor|GetAllActorsOfClass "/Game/Blueprints/PickUps/CheckPoint.CheckPoint_C"))
        (for _array_element_56 _outactors_56
          (bind _ascheckpoint_c_55 (Utilities|Casting|CastToCheckPoint _array_element_56))
          (if (== OtherActor _ascheckpoint_c_55)
            (Variables|Default|SetCheckPoint (Transformation|GetActorLocation))
            (Development|PrintString "Check Point Established")
            (Class|GameplayStatics|PlaySoundAttached "/Game/Audio/SetCheckPoint.SetCheckPoint" _mesh)
            (Variables|Default|SetHealth 5)
            (goto _label_3)))
        (bind _ascheckpoint_c_56 (Utilities|Casting|CastToCheckPoint _array_element_56))
        (if (== OtherActor _ascheckpoint_c_56)
          (Variables|Default|SetCheckPoint (Transformation|GetActorLocation))
          (Development|PrintString "Check Point Established")
          (Class|GameplayStatics|PlaySoundAttached "/Game/Audio/SetCheckPoint.SetCheckPoint" _mesh)
          (Variables|Default|SetHealth 5)
          (goto _label_3)))))
  (bind _outactors_57 (Actor|GetAllActorsOfClass "/Game/Blueprints/PickUps/LevelDest.LevelDest_C"))
  (for _array_element_57 _outactors_57
    (bind _asleveldest_c_8 (Utilities|Casting|CastToLevelDest _array_element_57))
    (if (== OtherActor _asleveldest_c_8)
      (Game|SpawnActorfromClass "/Game/Blueprints/ArrowPointer.ArrowPointer_C" (Math|Conversions|ToTransform(Vector) (Transformation|GetActorLocation)) false 0)
      (Development|PrintString "Desination Found")
      (Class|GameplayStatics|PlaySoundAttached "/Game/Audio/Director.Director" _mesh)
      (Actor|DestroyActor OtherActor :!label _label_4)
      (else
        (bind _outactors_58 (Actor|GetAllActorsOfClass "/Game/Blueprints/PickUps/JumpBoost.JumpBoost_C"))
        (for _array_element_58 _outactors_58
          (bind _asjumpboost_c_15 (Utilities|Casting|CastToJumpBoost _array_element_58))
          (if (== OtherActor _asjumpboost_c_15)
            (Variables|Default|SetJumpPower 3.0)
            (Development|PrintString "Booster Equipped")
            (Class|GameplayStatics|PlaySoundAttached "/Game/Audio/JumpBoost.JumpBoost" _mesh)
            (goto _label_4)
            (else
              (bind _outactors_59 (Actor|GetAllActorsOfClass "/Game/Blueprints/PickUps/CheckPoint.CheckPoint_C"))
              (for _array_element_59 _outactors_59
                (bind _ascheckpoint_c_57 (Utilities|Casting|CastToCheckPoint _array_element_59))
                (if (== OtherActor _ascheckpoint_c_57)
                  (Variables|Default|SetCheckPoint (Transformation|GetActorLocation))
                  (Development|PrintString "Check Point Established")
                  (Class|GameplayStatics|PlaySoundAttached "/Game/Audio/SetCheckPoint.SetCheckPoint" _mesh)
                  (Variables|Default|SetHealth 5)
                  (goto _label_4)))
              (bind _ascheckpoint_c_58 (Utilities|Casting|CastToCheckPoint _array_element_59))
              (if (== OtherActor _ascheckpoint_c_58)
                (Variables|Default|SetCheckPoint (Transformation|GetActorLocation))
                (Development|PrintString "Check Point Established")
                (Class|GameplayStatics|PlaySoundAttached "/Game/Audio/SetCheckPoint.SetCheckPoint" _mesh)
                (Variables|Default|SetHealth 5)
                (goto _label_4)))))
        (bind _outactors_60 (Actor|GetAllActorsOfClass "/Game/Blueprints/PickUps/CheckPoint.CheckPoint_C"))
        (for _array_element_60 _outactors_60
          (bind _ascheckpoint_c_59 (Utilities|Casting|CastToCheckPoint _array_element_60))
          (if (== OtherActor _ascheckpoint_c_59)
            (Variables|Default|SetCheckPoint (Transformation|GetActorLocation))
            (Development|PrintString "Check Point Established")
            (Class|GameplayStatics|PlaySoundAttached "/Game/Audio/SetCheckPoint.SetCheckPoint" _mesh)
            (Variables|Default|SetHealth 5)
            (goto _label_4)))
        (bind _ascheckpoint_c_60 (Utilities|Casting|CastToCheckPoint _array_element_60))
        (if (== OtherActor _ascheckpoint_c_60)
          (Variables|Default|SetCheckPoint (Transformation|GetActorLocation))
          (Development|PrintString "Check Point Established")
          (Class|GameplayStatics|PlaySoundAttached "/Game/Audio/SetCheckPoint.SetCheckPoint" _mesh)
          (Variables|Default|SetHealth 5)
          (goto _label_4)))))
  (bind _outactors_61 (Actor|GetAllActorsOfClass "/Game/Blueprints/PickUps/JumpBoost.JumpBoost_C"))
  (for _array_element_61 _outactors_61
    (bind _asjumpboost_c_16 (Utilities|Casting|CastToJumpBoost _array_element_61))
    (if (== OtherActor _asjumpboost_c_16)
      (Variables|Default|SetJumpPower 3.0)
      (Development|PrintString "Booster Equipped")
      (Class|GameplayStatics|PlaySoundAttached "/Game/Audio/JumpBoost.JumpBoost" _mesh)
      (Actor|DestroyActor OtherActor :!label _label_5)
      (else
        (bind _outactors_62 (Actor|GetAllActorsOfClass "/Game/Blueprints/PickUps/CheckPoint.CheckPoint_C"))
        (for _array_element_62 _outactors_62
          (bind _ascheckpoint_c_61 (Utilities|Casting|CastToCheckPoint _array_element_62))
          (if (== OtherActor _ascheckpoint_c_61)
            (Variables|Default|SetCheckPoint (Transformation|GetActorLocation))
            (Development|PrintString "Check Point Established")
            (Class|GameplayStatics|PlaySoundAttached "/Game/Audio/SetCheckPoint.SetCheckPoint" _mesh)
            (Variables|Default|SetHealth 5)
            (goto _label_5)))
        (bind _ascheckpoint_c_62 (Utilities|Casting|CastToCheckPoint _array_element_62))
        (if (== OtherActor _ascheckpoint_c_62)
          (Variables|Default|SetCheckPoint (Transformation|GetActorLocation))
          (Development|PrintString "Check Point Established")
          (Class|GameplayStatics|PlaySoundAttached "/Game/Audio/SetCheckPoint.SetCheckPoint" _mesh)
          (Variables|Default|SetHealth 5)
          (goto _label_5)))))
  (bind _outactors_63 (Actor|GetAllActorsOfClass "/Game/Blueprints/PickUps/CheckPoint.CheckPoint_C"))
  (for _array_element_63 _outactors_63
    (bind _ascheckpoint_c_63 (Utilities|Casting|CastToCheckPoint _array_element_63))
    (if (== OtherActor _ascheckpoint_c_63)
      (Variables|Default|SetCheckPoint (Transformation|GetActorLocation))
      (Development|PrintString "Check Point Established")
      (Class|GameplayStatics|PlaySoundAttached "/Game/Audio/SetCheckPoint.SetCheckPoint" _mesh)
      (Variables|Default|SetHealth 5)
      (Actor|DestroyActor OtherActor)))
  (bind _ascheckpoint_c_64 (Utilities|Casting|CastToCheckPoint _array_element_63))
  (if (== OtherActor _ascheckpoint_c_64)
    (Variables|Default|SetCheckPoint (Transformation|GetActorLocation))
    (Development|PrintString "Check Point Established")
    (Class|GameplayStatics|PlaySoundAttached "/Game/Audio/SetCheckPoint.SetCheckPoint" _mesh)
    (Variables|Default|SetHealth 5)
    (Actor|DestroyActor OtherActor)))

(event EventTick
  (params (DeltaSeconds :type Float%20%28single-precision%29))
  (bind _returnvalue (Transformation|GetVelocity))
  (bind _jumppower (Variables|Default|GetJumpPower))
  (bind _mesh (Variables|Character|GetMesh))
  (bind (_x _y) (Math|Vector|BreakVector _returnvalue))
  ;[1 1 1] Death Check
  (if (Variables|Default|GetGameOver)
    (Class|GameplayStatics|PlaySoundAttached "/Game/Audio/HeartContainerGet.HeartContainerGet" _mesh)
    (Audio|Components|Audio|Stop (stale EventAnyDamage _returnvalue))
    (elif (<= (Variables|Default|GetHealth) 0)
      (Class|GameplayStatics|PlaySoundAttached "/Game/Audio/Game_Over_-_The_Legend_of_Zelda-_Ocarina_of_Time.Game_Over_-_The_Legend_of_Zelda-_Ocarina_of_Time" _mesh)
      (Audio|Components|Audio|Stop (stale Custom|MusicTimer _returnvalue))
      (Actor|DestroyActor)
      (else
        ;[1 1 1] Respawn
        (if (<= (.Z (Math|Vector|BreakVector (Transformation|GetActorLocation))) -1.5e+02)
          (Class|GameplayStatics|PlaySoundAttached "/Game/Audio/Warp.Warp" _mesh)
          (Transformation|SetActorLocationAndRotation (Variables|Default|GetCheckPoint) (Variables|Default|GetStartRot))
          (Variables|Default|SetHealth (- (Variables|Default|GetHealth) 1))
          (else
            ;[1 1 1] Jetpack
            (if (Variables|Default|GetJetPack)
              (if (== (Transformation|GetVelocity) (Math|Vector|MakeVector _x _y 0.0))
                (Character|LaunchCharacter "0, 0,1000.000000" false false)
                (elif (>= (Variables|Default|GetFuel) 4)
                  (Character|LaunchCharacter (* (+ (* (Transformation|GetActorForwardVector) _jumppower) (* (Transformation|GetActorUpVector) _jumppower)) 1e+01) false false)
                  (Variables|Default|SetFuel (- (Variables|Default|GetFuel) 1))
                  (else
                    (Variables|Default|SetFuel 0)))))))))))

(event Input|ActionEvents|InputActionFire
  ;[1 1 1] Score
  (:Released
    (Variables|Default|SetScore (- (Variables|Default|GetScore) 1))))

(event Input|GamepadEvents|GamepadSpecialRight
  ;[1 1 1] Pausing
  (:Pressed
    (if (not (Variables|Default|GetGameOver))
      (Utilities|FlowControl|FlipFlop
        (:A
          (Game|SetGamePaused false))
        (:B
          (Game|SetGamePaused true))))))

(event Input|MouseEvents|RightMouseButton
  ;[1 1 1] Pausing
  (:Pressed
    (if (not (Variables|Default|GetGameOver))
      (Utilities|FlowControl|FlipFlop
        (:A
          (Game|SetGamePaused false))
        (:B
          (Game|SetGamePaused true))))))

(event Input|KeyboardEvents|SpaceBar
  ;[1 1 1] Jetpack
  (:Pressed
    (Variables|Default|SetJetPack true))
  (:Released
    (Variables|Default|SetJetPack false)))

(event Input|GamepadEvents|GamepadSpecialLeft
  ;[1 1 1] Pausing
  (:Pressed
    (Game|OpenLevel(byName) "Menu")))

(event Input|GamepadEvents|GamepadFaceButtonBottom
  ;[1 1 1] Jetpack
  (:Pressed
    (Variables|Default|SetJetPack true))
  (:Released
    (Variables|Default|SetJetPack false)))

(fn ConstructionScript)

(fn GetHealth
  (return (Variables|Default|GetHealth)))

(fn GetGameOver
  (return (Variables|Default|GetGameOver)))

(fn GetScore
  (return (Variables|Default|GetScore)))