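; Meteor actor that drifts around the player and triggers game over when its health runs out.
; Tick adds a small random positive X/Y offset, or resets it to world origin when too far from the player.
; Each Hit drains health; at zero it plays a sound, unpauses, sets GameOver on the character reference and destroys itself.
; BeginPlay starts looping move and rotate timers whose target functions are absent here.
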(event EventHit
  (params (MyComp :type Primitive%20Component%20Object%20Reference) (Other :type Actor%20Object%20Reference) (OtherComp :type Primitive%20Component%20Object%20Reference) (bSelfMoved :type Boolean) (HitLocation :type Vector :default "0, 0, 0") (HitNormal :type Vector :default "0, 0, 0") (NormalImpulse :type Vector :default "0, 0, 0") (Hit :type Hit%20Result%20Structure%20%28by%20ref%29))
  ;[1 1 1] Health Reduction
  (Variables|Default|SetHealth (- (Variables|Default|GetHealth) 1)))

(event EventTick
  (params (DeltaSeconds :type Float%20%28single-precision%29))
  (bind _returnvalue (Transformation|GetActorLocation))
  ;[1 1 1] Movement
  (if (< 5e+03 (Math|Vector|VectorLength (- (Transformation|GetActorLocation (Game|GetPlayerCharacter 0)) _returnvalue)))
    (Transformation|SetActorLocation "0, 0, 0" false)
    (else
      (Transformation|SetActorLocation (+ _returnvalue (Math|Vector|MakeVector (Math|Random|RandomFloat) (Math|Random|RandomFloat) 0.0)) false)))
  ;[1 1 1] DestroyState
  (if (<= (Variables|Default|GetHealth) 0)
    (Class|GameplayStatics|PlaySoundAttached "/Game/Audio/HeartContainerGet.HeartContainerGet" (Variables|Character|GetMesh))
    (Game|SetGamePaused false)
    (Variables|/Game/Blueprints/MyCharacter.MyCharacter_C|SetGameOver (Variables|Default|GetCharacterReference) true)
    (Actor|DestroyActor)))

(event EventBeginPlay
  ;[1 1 1] Set Up
  (Utilities|Time|SetTimerbyFunctionName 0 "MoveTimer" 0.5 true)
  (Utilities|Time|SetTimerbyFunctionName 0 "RotateTimer" 0.3 true))

(fn ConstructionScript)