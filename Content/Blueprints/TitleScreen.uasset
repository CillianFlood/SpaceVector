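; TitleScreen is a title actor that animates two components, Space and Vector, sliding in opposite directions along the X axis before removing itself.
; Each Tick moves Space toward positive X and Vector toward negative X by a fixed per-frame step, without scaling by delta time.
; Once Space reaches an X threshold, movement stops and the actor destroys itself after a short delay.
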(event EventTick
  (params (DeltaSeconds :type Float%20%28single-precision%29))
  (bind _space (Variables|Default|GetSpace))
  (bind _vector (Variables|Default|GetVector))
  (bind _returnvalue (Transformation|GetWorldLocation _space))
  (bind _returnvalue_2 (Transformation|GetWorldLocation _vector))
  (bind (_x _y _z) (Math|Vector|BreakVector _returnvalue))
  (bind (_x_2 _y_2 _z_2) (Math|Vector|BreakVector _returnvalue_2))
  (if (<= -3.3e+02 _x)
    (Utilities|FlowControl|Delay 3.0)
    (Actor|DestroyActor)
    (else
      (Transformation|SetWorldLocation _space (Math|Vector|MakeVector (+ _x 5.0) _y _z) false)
      (Transformation|SetWorldLocation _vector (Math|Vector|MakeVector (- _x_2 5.0) _y_2 _z_2) false))))

(fn ConstructionScript)