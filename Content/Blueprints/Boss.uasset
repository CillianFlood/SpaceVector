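; Boss actor that spins four spokes and tumbles on an axis re-rolled by timer, periodically firing BossAtack actors from the spokes.
; While its barrier is down, Tick scans all Projectiles by distance to the Core to apply damage.
; Each non-lethal hit toggles the barrier through a FlipFlop, toggled again by timer.
; Low health changes spoke speed and adds BossFire; death triggers random explosions, a delayed sound and destruction.
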(event Custom|ModeChange
  ;[1 1 1] ChangeMode
  (Variables|Default|SetMode (Math|Random|RandomIntegerinRange 1 3)))

(event Custom|Barrier
  (bind _core (Variables|Default|GetCore))
  ;[1 1 1] Barrier
  (Utilities|FlowControl|FlipFlop
    (:A
      (Rendering|Material|SetMaterial _core 0 "/Engine/EngineDebugMaterials/BoneWeightMaterial.BoneWeightMaterial")
      (Variables|Default|SetBarrierDown false))
    (:B
      (Rendering|Material|SetMaterial _core 0 "/Engine/EditorMaterials/WidgetGridVertexColorMaterial_Ma.WidgetGridVertexColorMaterial_Ma")
      (Variables|Default|SetBarrierDown true)))
  (if (== (Variables|Default|GetHealth) 10)
    (Variables|Default|SetSpeed 3.0)))

(event Custom|Fire
  ;[1 1 1] Fire
  (if (> (Variables|Default|GetHealth) 0)
    (Game|SpawnActorfromClass "/Game/Blueprints/BossAtack.BossAtack_C" (Transformation|GetSocketTransform (Variables|Default|GetSpoke1) "Socket" "RTS_World") false 0)
    (Game|SpawnActorfromClass "/Game/Blueprints/BossAtack.BossAtack_C" (Transformation|GetSocketTransform (Variables|Default|GetSpoke2) "Socket" "RTS_World") false 0)
    (Game|SpawnActorfromClass "/Game/Blueprints/BossAtack.BossAtack_C" (Transformation|GetSocketTransform (Variables|Default|GetSpoke3) "Socket" "RTS_World") false 0)
    (Game|SpawnActorfromClass "/Game/Blueprints/BossAtack.BossAtack_C" (Transformation|GetSocketTransform (Variables|Default|GetSpoke4) "Socket" "RTS_World") false 0)
    (if (<= (Variables|Default|GetHealth) 10)
      (Game|SpawnActorfromClass "/Game/Blueprints/BossFire.BossFire_C" (Transformation|GetSocketTransform (Variables|Default|GetCore) "None" "RTS_World") false 0))))

(event EventTick
  (params (DeltaSeconds :type Float%20%28single-precision%29))
  (bind _returnvalue (Transformation|GetActorLocation))
  (bind _returnvalue_2 (Math|Random|RandomFloatinRange -5e+02 5e+02))
  (bind _spoke1 (Variables|Default|GetSpoke1))
  (bind _spoke2 (Variables|Default|GetSpoke2))
  (bind _spoke3 (Variables|Default|GetSpoke3))
  (bind _spoke4 (Variables|Default|GetSpoke4))
  (bind _mode (Variables|Default|GetMode))
  (bind _core (Variables|Default|GetCore))
  (bind _returnvalue_3 (Transformation|GetWorldLocation _spoke3))
  (bind _returnvalue_4 (Transformation|GetWorldLocation _core))
  (bind _returnvalue_5 (Transformation|GetWorldLocation _spoke4))
  (bind _returnvalue_6 (Transformation|GetWorldLocation _spoke1))
  (bind _returnvalue_7 (Transformation|GetWorldLocation _spoke2))
  (bind (_x _y _z) (Math|Vector|BreakVector _returnvalue))
  (bind _returnvalue_8 (Transformation|GetWorldRotation _spoke1))
  (bind _returnvalue_9 (Transformation|GetWorldRotation _spoke4))
  (bind _returnvalue_10 (Transformation|GetWorldRotation _spoke2))
  (bind _returnvalue_11 (Transformation|GetWorldRotation _spoke3))
  (bind (_pitch _yaw _roll) (Class|KismetMathLibrary|BreakRot _returnvalue_9))
  (bind (_pitch_2 _yaw_2 _roll_2) (Class|KismetMathLibrary|BreakRot _returnvalue_8))
  (bind (_pitch_3 _yaw_3 _roll_3) (Class|KismetMathLibrary|BreakRot _returnvalue_10))
  (bind (_pitch_4 _yaw_4 _roll_4) (Class|KismetMathLibrary|BreakRot _returnvalue_11))
  (bind (_x_2 _y_2 _z_2) (Math|Vector|BreakVector _returnvalue_4))
  (bind (_x_3 _y_3 _z_3) (Math|Vector|BreakVector _returnvalue_6))
  (bind (_x_4 _y_4 _z_4) (Math|Vector|BreakVector _returnvalue_7))
  (bind (_x_5 _y_5 _z_5) (Math|Vector|BreakVector _returnvalue_3))
  (bind (_x_6 _y_6 _z_6) (Math|Vector|BreakVector _returnvalue_5))
  ;[1 1 1] SpinSpokes
  (if (> (Variables|Default|GetHealth) 0)
    (Transformation|SetWorldRotation _spoke1 (Class|KismetMathLibrary|MakeRot _pitch_2 (+ _yaw_2 (Variables|Default|GetSpeed)) _roll_2) false)
    (Transformation|SetWorldRotation _spoke2 (Class|KismetMathLibrary|MakeRot _pitch_3 (+ _yaw_3 (Variables|Default|GetSpeed)) _roll_3) false)
    (Transformation|SetWorldRotation _spoke3 (Class|KismetMathLibrary|MakeRot _pitch_4 (+ _yaw_4 (Variables|Default|GetSpeed)) _roll_4) false)
    (Transformation|SetWorldRotation _spoke4 (Class|KismetMathLibrary|MakeRot _pitch (+ _yaw (Variables|Default|GetSpeed)) _roll) false)
    ;[1 1 1] SpinSelf
    (if (== _mode 1)
      (Transformation|AddActorLocalRotation "0.000000,0.000000,1.000000" false)
      (elif (== 2 _mode)
        (Transformation|AddActorLocalRotation "1.000000,0.000000,0.000000" false)
        (else
          (Transformation|AddActorLocalRotation "0.000000,10.000000,0.000000" false))))
    ;[1 1 1] Damage Calc
    (if (Variables|Default|GetBarrierDown)
      (bind _outactors (Actor|GetAllActorsOfClass "/Game/Blueprints/Projectile.Projectile_C"))
      (for _array_element _outactors
        (bind _asprojectile_c (Utilities|Casting|CastToProjectile _array_element))
        (if (<= (Math|Vector|VectorLength (- (Transformation|GetWorldLocation (Variables|Default|GetCore)) (Transformation|GetActorLocation _asprojectile_c))) 2e+02)
          (Variables|Default|SetHealth (- (Variables|Default|GetHealth) 1))
          (Actor|DestroyActor _asprojectile_c)
          (Game|SpawnActorfromClass "/Game/Blueprints/SilentExplosion.SilentExplosion_C" (Math|Conversions|ToTransform(Vector) (Math|Vector|MakeVector _x _y (+ 1.5e+02 _z))) false 0)
          (if (<= (Variables|Default|GetHealth) 0)
            (Rendering|Material|SetMaterial _core 0 "/Engine/MapTemplates/Materials/BasicAsset01.BasicAsset01")
            (Utilities|FlowControl|Delay 5.0)
            (Class|GameplayStatics|PlaySoundAttached "/Game/Audio/HeartContainerGet.HeartContainerGet" (Variables|Default|GetSkeletalMesh1))
            (Actor|DestroyActor)
            (else
              ;[1 1 1] Barrier
              (Utilities|Time|SetTimerbyFunctionName 0 "Barrier" 5.0)
              (Utilities|FlowControl|FlipFlop
                (:A
                  (Rendering|Material|SetMaterial _core 0 "/Engine/EngineDebugMaterials/BoneWeightMaterial.BoneWeightMaterial")
                  (Variables|Default|SetBarrierDown false))
                (:B
                  (Rendering|Material|SetMaterial _core 0 "/Engine/EditorMaterials/WidgetGridVertexColorMaterial_Ma.WidgetGridVertexColorMaterial_Ma")
                  (Variables|Default|SetBarrierDown true)))
              (if (== (Variables|Default|GetHealth) 10)
                (Variables|Default|SetSpeed 3.0)))))))
    (else
      ;[1 1 1] DeathAnimation
      (Utilities|FlowControl|Delay 0.8)
      (Game|SpawnActorfromClass "/Game/Blueprints/SilentExplosion.SilentExplosion_C" (Math|Conversions|ToTransform(Vector) (Math|Vector|MakeVector (+ _x_3 _returnvalue_2) (+ _y_3 _returnvalue_2) (+ _z_3 _returnvalue_2))) false 0)
      (Game|SpawnActorfromClass "/Game/Blueprints/SilentExplosion.SilentExplosion_C" (Math|Conversions|ToTransform(Vector) (Math|Vector|MakeVector (+ _x_4 _returnvalue_2) (+ _y_4 _returnvalue_2) (+ _z_4 _returnvalue_2))) false 0)
      (Game|SpawnActorfromClass "/Game/Blueprints/SilentExplosion.SilentExplosion_C" (Math|Conversions|ToTransform(Vector) (Math|Vector|MakeVector (+ _x_5 _returnvalue_2) (+ _y_5 _returnvalue_2) (+ _z_5 _returnvalue_2))) false 0)
      (Game|SpawnActorfromClass "/Game/Blueprints/SilentExplosion.SilentExplosion_C" (Math|Conversions|ToTransform(Vector) (Math|Vector|MakeVector (+ _x_6 _returnvalue_2) (+ _y_6 _returnvalue_2) (+ _z_6 _returnvalue_2))) false 0)
      (Game|SpawnActorfromClass "/Game/Blueprints/SilentExplosion.SilentExplosion_C" (Math|Conversions|ToTransform(Vector) (Math|Vector|MakeVector (+ _x_2 _returnvalue_2) (+ _y_2 _returnvalue_2) (+ _z_2 _returnvalue_2))) false 0))))

(event EventBeginPlay
  ;[1 1 1] SetUp
  (Utilities|Time|SetTimerbyFunctionName 0 "ModeChange" 8.0 true)
  (Utilities|Time|SetTimerbyFunctionName 0 "Fire" 5.0 true))

(fn ConstructionScript)