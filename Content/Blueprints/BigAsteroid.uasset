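; BigAsteroid is a large asteroid that homes in on the player character and splits when struck.
; Tick lerps it toward the player, damaging them and destroying itself at close range, with a timed sound and "Danger!" warning when nearby.
; Hit or overlap destroys both actors, spawning two offset Asteroids and silent explosions.
; It can also remove itself on game over.
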(event Custom|AlarmTimer
  ;[1 1 1] Alarm
  (Audio|PlaySoundatLocation "/Game/Audio/Alarm.Alarm" (Transformation|GetActorLocation) 0.5)
  (Development|PrintString "Danger!" true true "(R=1.000000,G=0.009182,B=0.000000,A=1.000000)"))

(event EventHit
  (params (MyComp :type Primitive%20Component%20Object%20Reference) (Other :type Actor%20Object%20Reference) (OtherComp :type Primitive%20Component%20Object%20Reference) (bSelfMoved :type Boolean) (HitLocation :type Vector :default "0, 0, 0") (HitNormal :type Vector :default "0, 0, 0") (NormalImpulse :type Vector :default "0, 0, 0") (Hit :type Hit%20Result%20Structure%20%28by%20ref%29))
  (bind _returnvalue (Transformation|GetActorLocation))
  (bind (_x _y _z) (Math|Vector|BreakVector _returnvalue))
  (bind (_x_2 _y_2 _z_2) (Math|Vector|BreakVector _returnvalue))
  (bind _returnvalue_2 (+ _y_2 -5e+01))
  (bind _returnvalue_3 (+ _z_2 -5e+01))
  (bind _returnvalue_4 (+ _y 5e+01))
  (bind _returnvalue_5 (+ _z 5e+01))
  (bind _returnvalue_6 (+ _x_2 -5e+01))
  (bind _returnvalue_7 (+ _x 5e+01))
  (bind _returnvalue_8 (Math|Vector|MakeVector _returnvalue_6 _returnvalue_2 _returnvalue_3))
  (bind _returnvalue_9 (Math|Vector|MakeVector _returnvalue_7 _returnvalue_4 _returnvalue_5))
  (bind _returnvalue_10 (Math|Conversions|ToTransform(Vector) _returnvalue_8))
  (bind _returnvalue_11 (Math|Conversions|ToTransform(Vector) _returnvalue_9))
  ;[1 1 1] Collision Response
  (Actor|DestroyActor Other)
  (Game|SpawnActorfromClass "/Game/Blueprints/Asteroid.Asteroid_C" _returnvalue_10 false 0)
  (Game|SpawnActorfromClass "/Game/Blueprints/Asteroid.Asteroid_C" _returnvalue_11 false 0)
  (Game|SpawnActorfromClass "/Game/Blueprints/SilentExplosion.SilentExplosion_C" (Math|Conversions|ToTransform(Vector) (Transformation|GetActorLocation)) false 0)
  (Game|SpawnActorfromClass "/Game/Blueprints/SilentExplosion.SilentExplosion_C" _returnvalue_11 false 0)
  (Game|SpawnActorfromClass "/Game/Blueprints/SilentExplosion.SilentExplosion_C" _returnvalue_10 false 0)
  (Actor|DestroyActor))

(event EventTick
  (params (DeltaSeconds :type Float%20%28single-precision%29))
  (bind _returnvalue (Transformation|GetActorLocation))
  (bind _returnvalue_2 (Game|GetPlayerCharacter 0))
  (bind _speed (Variables|Default|GetSpeed))
  (bind _returnvalue_3 (Transformation|GetActorLocation _returnvalue_2))
  (bind _returnvalue_4 (* DeltaSeconds _speed))
  (bind _returnvalue_5 (Math|Vector|Lerp(Vector) _returnvalue _returnvalue_3 _returnvalue_4))
  (bind _returnvalue_6 (- _returnvalue _returnvalue_3))
  (bind _returnvalue_7 (Math|Vector|VectorLength _returnvalue_6))
  ;[1 1 1] Movement
  (Transformation|SetActorLocation _returnvalue_5 false)
  (Transformation|SetActorRotation (Math|Rotator|FindLookatRotation _returnvalue_5 _returnvalue_3))
  ;[1 1 1] Apply Damage
  (if (<= _returnvalue_7 3.5e+02)
    (Game|Damage|ApplyDamage (Game|GetPlayerCharacter 0) 3.0 (Pawn|GetController) self "/Script/Engine.DamageType")
    (Actor|DestroyActor)
    (else
      ;[1 1 1] Alarm
      (if (and (<= _returnvalue_7 1e+03) (Math|Boolean|Equal(Boolean) (Class|KismetSystemLibrary|IsTimerActive 0 "AlarmTimer") false))
        (Utilities|Time|SetTimerbyFunctionName 0 "AlarmTimer" 0.7)
        (elif (Variables|/Game/Blueprints/MyCharacter.MyCharacter_C|GetGameOver (Variables|Default|GetCharacterReference))
          (Actor|DestroyActor))))))

(event EventActorBeginOverlap
  (params (OtherActor :type Actor%20Object%20Reference))
  (bind _returnvalue (Transformation|GetActorLocation))
  (bind (_x _y _z) (Math|Vector|BreakVector _returnvalue))
  (bind (_x_2 _y_2 _z_2) (Math|Vector|BreakVector _returnvalue))
  (bind _returnvalue_2 (+ _y_2 -5e+01))
  (bind _returnvalue_3 (+ _z_2 -5e+01))
  (bind _returnvalue_4 (+ _y 5e+01))
  (bind _returnvalue_5 (+ _z 5e+01))
  (bind _returnvalue_6 (+ _x_2 -5e+01))
  (bind _returnvalue_7 (+ _x 5e+01))
  (bind _returnvalue_8 (Math|Vector|MakeVector _returnvalue_6 _returnvalue_2 _returnvalue_3))
  (bind _returnvalue_9 (Math|Vector|MakeVector _returnvalue_7 _returnvalue_4 _returnvalue_5))
  (bind _returnvalue_10 (Math|Conversions|ToTransform(Vector) _returnvalue_8))
  (bind _returnvalue_11 (Math|Conversions|ToTransform(Vector) _returnvalue_9))
  ;[1 1 1] Collision Response
  (Actor|DestroyActor (stale EventHit Other))
  (Game|SpawnActorfromClass "/Game/Blueprints/Asteroid.Asteroid_C" _returnvalue_10 false 0)
  (Game|SpawnActorfromClass "/Game/Blueprints/Asteroid.Asteroid_C" _returnvalue_11 false 0)
  (Game|SpawnActorfromClass "/Game/Blueprints/SilentExplosion.SilentExplosion_C" (Math|Conversions|ToTransform(Vector) (Transformation|GetActorLocation)) false 0)
  (Game|SpawnActorfromClass "/Game/Blueprints/SilentExplosion.SilentExplosion_C" _returnvalue_11 false 0)
  (Game|SpawnActorfromClass "/Game/Blueprints/SilentExplosion.SilentExplosion_C" _returnvalue_10 false 0)
  (Actor|DestroyActor))

(fn ConstructionScript)