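; ArrowPointer is an actor that hovers near the player and points toward the LevelWarper.
; Every tick it finds all LevelWarper actors and, for each, snaps to a fixed offset from the player and rotates with a look-at toward it, so the last one found sets the facing.
; A timeline, played from the same loop, adds a local offset to animate the arrow.
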(event EventTick
  (params (DeltaSeconds :type Float%20%28single-precision%29))
  (bind _returnvalue (Game|GetPlayerCharacter 0))
  (bind _returnvalue_2 (Transformation|GetActorLocation _returnvalue))
  (bind (_x _y _z) (Math|Vector|BreakVector _returnvalue_2))
  ;[1 1 1] Update
  (bind _outactors (Actor|GetAllActorsOfClass "/Game/Blueprints/LevelWarper.LevelWarper_C"))
  (for _array_element _outactors
    (Transformation|SetActorLocation (Math|Vector|MakeVector _x (+ _y 5e+01) (+ _z 5e+01)) false)
    (Transformation|SetActorRotation (Math|Rotator|FindLookatRotation (Math|Vector|Lerp(Vector) (Transformation|GetActorLocation) (Transformation|GetActorLocation _array_element) DeltaSeconds) (Transformation|GetActorLocation _array_element)))
    (bind _newtrack_0 (Timeline|Timeline_0 Play)
      (:Update
        (Transformation|AddActorLocalOffset _newtrack_0 false)))))

(fn ConstructionScript)