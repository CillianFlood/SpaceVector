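; Boss attack projectile that homes on a snapshot of the player's location taken at BeginPlay, not on the moving player.
; Tick lerps it toward that point and applies damage by distance check to the live player position, then self-destructs.
; Overlap or hit destroys the other actor, spawns a SilentExplosion and removes the projectile.
; A short lifespan timer or a missing player also destroys it.
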(event Custom|LifeSpan
  ;[1 1 1] LifeSpan
  (Actor|DestroyActor))

(event EventBeginPlay
  ;[1 1 1] SetUp
  (Transformation|SetActorRotation (Math|Rotator|FindLookatRotation (Math|Vector|Lerp(Vector) (Transformation|GetActorLocation) (Variables|Default|GetPlayerLoc) (* (stale EventTick DeltaSeconds) (Variables|Default|GetSpeed))) (Variables|Default|GetPlayerLoc)))
  (Variables|Default|SetPlayerLoc (Transformation|GetActorLocation (Game|GetPlayerCharacter 0)))
  (Utilities|Time|SetTimerbyFunctionName 0 "LifeSpan" 3.0))

(event EventHit
  (params (MyComp :type Primitive%20Component%20Object%20Reference) (Other :type Actor%20Object%20Reference) (OtherComp :type Primitive%20Component%20Object%20Reference) (bSelfMoved :type Boolean) (HitLocation :type Vector :default "0, 0, 0") (HitNormal :type Vector :default "0, 0, 0") (NormalImpulse :type Vector :default "0, 0, 0") (Hit :type Hit%20Result%20Structure%20%28by%20ref%29))
  ;[1 1 1] Collision Response
  (Actor|DestroyActor Other)
  (Game|SpawnActorfromClass "/Game/Blueprints/SilentExplosion.SilentExplosion_C" (Math|Conversions|ToTransform(Vector) (Transformation|GetActorLocation)) false 0)
  (Actor|DestroyActor))

(event EventTick
  (params (DeltaSeconds :type Float%20%28single-precision%29))
  (bind _returnvalue (Transformation|GetActorLocation))
  ;[1 1 1] Movement
  (if (== (Game|GetPlayerCharacter 0) 0)
    (Actor|DestroyActor)
    (else
      (Transformation|SetActorLocation (Math|Vector|Lerp(Vector) _returnvalue (Variables|Default|GetPlayerLoc) (* DeltaSeconds (Variables|Default|GetSpeed))) false)
      ;[1 1 1] Apply Damage
      (if (<= (Math|Vector|VectorLength (- _returnvalue (Transformation|GetActorLocation (Game|GetPlayerCharacter 0)))) 1.5e+02)
        (Game|Damage|ApplyDamage (Game|GetPlayerCharacter 0) 1.0 (Pawn|GetController) self "/Script/Engine.DamageType")
        (Actor|DestroyActor)))))

(event EventActorBeginOverlap
  (params (OtherActor :type Actor%20Object%20Reference))
  ;[1 1 1] Collision Response
  (Actor|DestroyActor (stale EventHit Other))
  (Game|SpawnActorfromClass "/Game/Blueprints/SilentExplosion.SilentExplosion_C" (Math|Conversions|ToTransform(Vector) (Transformation|GetActorLocation)) false 0)
  (Actor|DestroyActor))

(fn ConstructionScript)