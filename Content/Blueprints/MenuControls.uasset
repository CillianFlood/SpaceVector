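; MenuControls handles gamepad navigation of a level-select menu with six entries: three numbered levels, Boss, Tutorial and Survival.
; D-pad and left-stick releases step a wrapping LevelSelector index down (left/up) or up (right/down).
; Each step moves every LevelSelector actor to a hard-coded relative location for that index.
; The bottom face button or right special button opens the matching level by name.
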(event Input|GamepadEvents|GamepadDPadDown
  ;[1 1 1] Increase Level Selector
  (:Released
    (if (>= (Variables|Default|GetLevelSelector) 6)
      (Variables|Default|SetLevelSelector 1)
      (else
        (Variables|Default|SetLevelSelector (+ (Variables|Default|GetLevelSelector) 1))))
    ;[1 1 1] Position Selector
    (bind _outactors (Actor|GetAllActorsOfClass "/Game/Blueprints/LevelSelector.LevelSelector_C"))
    (for _array_element _outactors
      (bind _aslevelselector_c (Utilities|Casting|CastToLevelSelector _array_element))
      (if (== (Variables|Default|GetLevelSelector) 1)
        (Transformation|SetActorRelativeLocation _aslevelselector_c "-350.000000,-296.000000,467.000000")
        (elif (== (Variables|Default|GetLevelSelector) 2)
          (Transformation|SetActorRelativeLocation _aslevelselector_c "-150.000000,-296.000000,467.000000" true)
          (elif (== (Variables|Default|GetLevelSelector) 3)
            (Transformation|SetActorRelativeLocation _aslevelselector_c "50.000000,-296.000000,467.000000")
            (elif (== (Variables|Default|GetLevelSelector) 4)
              (Transformation|SetActorRelativeLocation _aslevelselector_c "225.000000,-296.000000,467.000000")
              (elif (== (Variables|Default|GetLevelSelector) 5)
                (Transformation|SetActorRelativeLocation _aslevelselector_c "-311.000000,-200.000000,227.000000")
                (else
                  (Transformation|SetActorRelativeLocation _aslevelselector_c "50.000000,-200.000000,227.000000"))))))))))

(event Input|GamepadEvents|GamepadDPadUp
  ;[1 1 1] Decrease Level Selector
  (:Released
    (if (<= (Variables|Default|GetLevelSelector) 1)
      (Variables|Default|SetLevelSelector 6)
      (else
        (Variables|Default|SetLevelSelector (- (Variables|Default|GetLevelSelector) 1))))
    ;[1 1 1] Position Selector
    (bind _outactors (Actor|GetAllActorsOfClass "/Game/Blueprints/LevelSelector.LevelSelector_C"))
    (for _array_element _outactors
      (bind _aslevelselector_c (Utilities|Casting|CastToLevelSelector _array_element))
      (if (== (Variables|Default|GetLevelSelector) 1)
        (Transformation|SetActorRelativeLocation _aslevelselector_c "-350.000000,-296.000000,467.000000")
        (elif (== (Variables|Default|GetLevelSelector) 2)
          (Transformation|SetActorRelativeLocation _aslevelselector_c "-150.000000,-296.000000,467.000000" true)
          (elif (== (Variables|Default|GetLevelSelector) 3)
            (Transformation|SetActorRelativeLocation _aslevelselector_c "50.000000,-296.000000,467.000000")
            (elif (== (Variables|Default|GetLevelSelector) 4)
              (Transformation|SetActorRelativeLocation _aslevelselector_c "225.000000,-296.000000,467.000000")
              (elif (== (Variables|Default|GetLevelSelector) 5)
                (Transformation|SetActorRelativeLocation _aslevelselector_c "-311.000000,-200.000000,227.000000")
                (else
                  (Transformation|SetActorRelativeLocation _aslevelselector_c "50.000000,-200.000000,227.000000"))))))))))

(event Input|GamepadEvents|GamepadDPadLeft
  ;[1 1 1] Decrease Level Selector
  (:Released
    (if (<= (Variables|Default|GetLevelSelector) 1)
      (Variables|Default|SetLevelSelector 6)
      (else
        (Variables|Default|SetLevelSelector (- (Variables|Default|GetLevelSelector) 1))))
    ;[1 1 1] Position Selector
    (bind _outactors (Actor|GetAllActorsOfClass "/Game/Blueprints/LevelSelector.LevelSelector_C"))
    (for _array_element _outactors
      (bind _aslevelselector_c (Utilities|Casting|CastToLevelSelector _array_element))
      (if (== (Variables|Default|GetLevelSelector) 1)
        (Transformation|SetActorRelativeLocation _aslevelselector_c "-350.000000,-296.000000,467.000000")
        (elif (== (Variables|Default|GetLevelSelector) 2)
          (Transformation|SetActorRelativeLocation _aslevelselector_c "-150.000000,-296.000000,467.000000" true)
          (elif (== (Variables|Default|GetLevelSelector) 3)
            (Transformation|SetActorRelativeLocation _aslevelselector_c "50.000000,-296.000000,467.000000")
            (elif (== (Variables|Default|GetLevelSelector) 4)
              (Transformation|SetActorRelativeLocation _aslevelselector_c "225.000000,-296.000000,467.000000")
              (elif (== (Variables|Default|GetLevelSelector) 5)
                (Transformation|SetActorRelativeLocation _aslevelselector_c "-311.000000,-200.000000,227.000000")
                (else
                  (Transformation|SetActorRelativeLocation _aslevelselector_c "50.000000,-200.000000,227.000000"))))))))))

(event Input|GamepadEvents|GamepadDPadRight
  ;[1 1 1] Increase Level Selector
  (:Released
    (if (>= (Variables|Default|GetLevelSelector) 6)
      (Variables|Default|SetLevelSelector 1)
      (else
        (Variables|Default|SetLevelSelector (+ (Variables|Default|GetLevelSelector) 1))))
    ;[1 1 1] Position Selector
    (bind _outactors (Actor|GetAllActorsOfClass "/Game/Blueprints/LevelSelector.LevelSelector_C"))
    (for _array_element _outactors
      (bind _aslevelselector_c (Utilities|Casting|CastToLevelSelector _array_element))
      (if (== (Variables|Default|GetLevelSelector) 1)
        (Transformation|SetActorRelativeLocation _aslevelselector_c "-350.000000,-296.000000,467.000000")
        (elif (== (Variables|Default|GetLevelSelector) 2)
          (Transformation|SetActorRelativeLocation _aslevelselector_c "-150.000000,-296.000000,467.000000" true)
          (elif (== (Variables|Default|GetLevelSelector) 3)
            (Transformation|SetActorRelativeLocation _aslevelselector_c "50.000000,-296.000000,467.000000")
            (elif (== (Variables|Default|GetLevelSelector) 4)
              (Transformation|SetActorRelativeLocation _aslevelselector_c "225.000000,-296.000000,467.000000")
              (elif (== (Variables|Default|GetLevelSelector) 5)
                (Transformation|SetActorRelativeLocation _aslevelselector_c "-311.000000,-200.000000,227.000000")
                (else
                  (Transformation|SetActorRelativeLocation _aslevelselector_c "50.000000,-200.000000,227.000000"))))))))))

(event Input|GamepadEvents|GamepadFaceButtonBottom
  (bind _levelselector (Variables|Default|GetLevelSelector))
  ;[1 1 1] LoadLevel
  (:Pressed
    (if (== _levelselector 1)
      (Game|OpenLevel(byName) "level1")
      (elif (== _levelselector 2)
        (Game|OpenLevel(byName) "level2")
        (elif (== _levelselector 3)
          (Game|OpenLevel(byName) "level3")
          (elif (== _levelselector 4)
            (Game|OpenLevel(byName) "Boss")
            (elif (== _levelselector 5)
              (Game|OpenLevel(byName) "Tutorial")
              (else
                (Game|OpenLevel(byName) "Survival")))))))))

(event Input|GamepadEvents|GamepadSpecialRight
  (bind _levelselector (Variables|Default|GetLevelSelector))
  ;[1 1 1] LoadLevel
  (:Pressed
    (if (== _levelselector 1)
      (Game|OpenLevel(byName) "level1")
      (elif (== _levelselector 2)
        (Game|OpenLevel(byName) "level2")
        (elif (== _levelselector 3)
          (Game|OpenLevel(byName) "level3")
          (elif (== _levelselector 4)
            (Game|OpenLevel(byName) "Boss")
            (elif (== _levelselector 5)
              (Game|OpenLevel(byName) "Tutorial")
              (else
                (Game|OpenLevel(byName) "Survival")))))))))

(event Input|GamepadEvents|GamepadLeftStickRight
  ;[1 1 1] Increase Level Selector
  (:Released
    (if (>= (Variables|Default|GetLevelSelector) 6)
      (Variables|Default|SetLevelSelector 1)
      (else
        (Variables|Default|SetLevelSelector (+ (Variables|Default|GetLevelSelector) 1))))
    ;[1 1 1] Position Selector
    (bind _outactors (Actor|GetAllActorsOfClass "/Game/Blueprints/LevelSelector.LevelSelector_C"))
    (for _array_element _outactors
      (bind _aslevelselector_c (Utilities|Casting|CastToLevelSelector _array_element))
      (if (== (Variables|Default|GetLevelSelector) 1)
        (Transformation|SetActorRelativeLocation _aslevelselector_c "-350.000000,-296.000000,467.000000")
        (elif (== (Variables|Default|GetLevelSelector) 2)
          (Transformation|SetActorRelativeLocation _aslevelselector_c "-150.000000,-296.000000,467.000000" true)
          (elif (== (Variables|Default|GetLevelSelector) 3)
            (Transformation|SetActorRelativeLocation _aslevelselector_c "50.000000,-296.000000,467.000000")
            (elif (== (Variables|Default|GetLevelSelector) 4)
              (Transformation|SetActorRelativeLocation _aslevelselector_c "225.000000,-296.000000,467.000000")
              (elif (== (Variables|Default|GetLevelSelector) 5)
                (Transformation|SetActorRelativeLocation _aslevelselector_c "-311.000000,-200.000000,227.000000")
                (else
                  (Transformation|SetActorRelativeLocation _aslevelselector_c "50.000000,-200.000000,227.000000"))))))))))

(event Input|GamepadEvents|GamepadLeftStickDown
  ;[1 1 1] Increase Level Selector
  (:Released
    (if (>= (Variables|Default|GetLevelSelector) 6)
      (Variables|Default|SetLevelSelector 1)
      (else
        (Variables|Default|SetLevelSelector (+ (Variables|Default|GetLevelSelector) 1))))
    ;[1 1 1] Position Selector
    (bind _outactors (Actor|GetAllActorsOfClass "/Game/Blueprints/LevelSelector.LevelSelector_C"))
    (for _array_element _outactors
      (bind _aslevelselector_c (Utilities|Casting|CastToLevelSelector _array_element))
      (if (== (Variables|Default|GetLevelSelector) 1)
        (Transformation|SetActorRelativeLocation _aslevelselector_c "-350.000000,-296.000000,467.000000")
        (elif (== (Variables|Default|GetLevelSelector) 2)
          (Transformation|SetActorRelativeLocation _aslevelselector_c "-150.000000,-296.000000,467.000000" true)
          (elif (== (Variables|Default|GetLevelSelector) 3)
            (Transformation|SetActorRelativeLocation _aslevelselector_c "50.000000,-296.000000,467.000000")
            (elif (== (Variables|Default|GetLevelSelector) 4)
              (Transformation|SetActorRelativeLocation _aslevelselector_c "225.000000,-296.000000,467.000000")
              (elif (== (Variables|Default|GetLevelSelector) 5)
                (Transformation|SetActorRelativeLocation _aslevelselector_c "-311.000000,-200.000000,227.000000")
                (else
                  (Transformation|SetActorRelativeLocation _aslevelselector_c "50.000000,-200.000000,227.000000"))))))))))

(event Input|GamepadEvents|GamepadLeftStickLeft
  ;[1 1 1] Decrease Level Selector
  (:Released
    (if (<= (Variables|Default|GetLevelSelector) 1)
      (Variables|Default|SetLevelSelector 6)
      (else
        (Variables|Default|SetLevelSelector (- (Variables|Default|GetLevelSelector) 1))))
    ;[1 1 1] Position Selector
    (bind _outactors (Actor|GetAllActorsOfClass "/Game/Blueprints/LevelSelector.LevelSelector_C"))
    (for _array_element _outactors
      (bind _aslevelselector_c (Utilities|Casting|CastToLevelSelector _array_element))
      (if (== (Variables|Default|GetLevelSelector) 1)
        (Transformation|SetActorRelativeLocation _aslevelselector_c "-350.000000,-296.000000,467.000000")
        (elif (== (Variables|Default|GetLevelSelector) 2)
          (Transformation|SetActorRelativeLocation _aslevelselector_c "-150.000000,-296.000000,467.000000" true)
          (elif (== (Variables|Default|GetLevelSelector) 3)
            (Transformation|SetActorRelativeLocation _aslevelselector_c "50.000000,-296.000000,467.000000")
            (elif (== (Variables|Default|GetLevelSelector) 4)
              (Transformation|SetActorRelativeLocation _aslevelselector_c "225.000000,-296.000000,467.000000")
              (elif (== (Variables|Default|GetLevelSelector) 5)
                (Transformation|SetActorRelativeLocation _aslevelselector_c "-311.000000,-200.000000,227.000000")
                (else
                  (Transformation|SetActorRelativeLocation _aslevelselector_c "50.000000,-200.000000,227.000000"))))))))))

(event Input|GamepadEvents|GamepadLeftStickUp
  ;[1 1 1] Decrease Level Selector
  (:Released
    (if (<= (Variables|Default|GetLevelSelector) 1)
      (Variables|Default|SetLevelSelector 6)
      (else
        (Variables|Default|SetLevelSelector (- (Variables|Default|GetLevelSelector) 1))))
    ;[1 1 1] Position Selector
    (bind _outactors (Actor|GetAllActorsOfClass "/Game/Blueprints/LevelSelector.LevelSelector_C"))
    (for _array_element _outactors
      (bind _aslevelselector_c (Utilities|Casting|CastToLevelSelector _array_element))
      (if (== (Variables|Default|GetLevelSelector) 1)
        (Transformation|SetActorRelativeLocation _aslevelselector_c "-350.000000,-296.000000,467.000000")
        (elif (== (Variables|Default|GetLevelSelector) 2)
          (Transformation|SetActorRelativeLocation _aslevelselector_c "-150.000000,-296.000000,467.000000" true)
          (elif (== (Variables|Default|GetLevelSelector) 3)
            (Transformation|SetActorRelativeLocation _aslevelselector_c "50.000000,-296.000000,467.000000")
            (elif (== (Variables|Default|GetLevelSelector) 4)
              (Transformation|SetActorRelativeLocation _aslevelselector_c "225.000000,-296.000000,467.000000")
              (elif (== (Variables|Default|GetLevelSelector) 5)
                (Transformation|SetActorRelativeLocation _aslevelselector_c "-311.000000,-200.000000,227.000000")
                (else
                  (Transformation|SetActorRelativeLocation _aslevelselector_c "50.000000,-200.000000,227.000000"))))))))))

(fn ConstructionScript)